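; Player shield component that shows itself for a timed active period and blocks reactivation until its cooldown timer ends.
; ActivateShield starts separate active and cooldown timers, while DeactivateShield hides the component and signals OnShieldDeactivation.
; Getters report active status and cooldown progress from those timers.
; Despite its name, ReduceCooldown restarts the active timer with a shortened, clamped time and leaves the cooldown timer untouched.
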(event `DeactivateShield`
  (`self.SetVisibility` false)
  (`self.OnShieldDeactivation`))

(event `SetCanActivate`
  (set `self.bCanActivate` true))

(fn `ActivateShield`
  (params (CustomTime :type "Float (double-precision)"))
  (returns (bSuccess :type Boolean))
  (if (`KismetSystemLibrary.K2_IsTimerActiveHandle` (`self.CooldownTimer`))
    (return false)
    (else
      (bind _returnvalue (`KismetSystemLibrary.K2_SetTimerDelegate` (`|CreateDelegate` :!event `DeactivateShield`) (`KismetMathLibrary.SelectFloat` CustomTime (`self.DefaultActiveTime`) (> CustomTime 0.0))))
      (set `self.ActiveTimer` _returnvalue)
      (bind _returnvalue_2 (`KismetSystemLibrary.K2_SetTimerDelegate` (`|CreateDelegate` :!event `SetCanActivate`) (`self.DefaultCooldownTime`)))
      (set `self.CooldownTimer` _returnvalue_2)
      (`self.SetVisibility` true)
      (return true))))

(fn `GetActiveStatus`
  (returns (bIsActive :type Boolean))
  (return (`KismetSystemLibrary.K2_IsTimerActiveHandle` (`self.ActiveTimer`))))

(fn `GetShieldCooldownPercent`
  (returns (ShieldPercent :type "Float (double-precision)"))
  (bind _defaultcooldowntime (`self.DefaultCooldownTime`))
  (return (`KismetMathLibrary.SelectFloat` (/ (`KismetSystemLibrary.K2_GetTimerElapsedTimeHandle` (`self.CooldownTimer`)) _defaultcooldowntime) (/ _defaultcooldowntime _defaultcooldowntime) (`KismetSystemLibrary.K2_IsTimerActiveHandle` (`self.CooldownTimer`)))))

(fn `ReduceCooldown`
  (params (CustomCooldownReduction :type "Float (double-precision)"))
  (bind _activetimer (`self.ActiveTimer`))
  (bind _returnvalue (`KismetMathLibrary.SelectFloat` CustomCooldownReduction (`self.DefaultCooldownReduction`) (> CustomCooldownReduction 0.0)))
  (`KismetSystemLibrary.K2_PauseTimerHandle` _activetimer)
  (bind _returnvalue_2 (`KismetSystemLibrary.K2_SetTimerDelegate` (`|CreateDelegate` :!event `DeactivateShield`) (`KismetMathLibrary.FClamp` (- (`KismetSystemLibrary.K2_GetTimerRemainingTimeHandle` _activetimer) _returnvalue) 0.1 _returnvalue)))
  (set `self.ActiveTimer` _returnvalue_2))