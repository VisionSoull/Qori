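; BP_Shield is a timed player shield actor that shows its sphere when activated and stores the damageable owner it serves.
; Activate starts a timer using a positive custom time or the default, after which Deactivate calls RemoveShield on the owner and destroys the actor.
; ReduceCooldown restarts that timer with one second less remaining.
; GetShieldCooldownPercent divides timer elapsed time by the default duration, even for custom times, returning full when inactive.
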(event `self.ReceiveBeginPlay`)

(fn `Activate`
  (params (CustomTime :type "Float (double-precision)") (DamageableOwner :type "/Game/Blueprints/DamageSystem/BPI_Damageable Interface"))
  (set `self.Damageable Owner` DamageableOwner)
  (bind _returnvalue (`KismetSystemLibrary.K2_SetTimer` null "Deactivate" (`KismetMathLibrary.SelectFloat` CustomTime (`self.DefaultActiveTime`) (> CustomTime 0.0))))
  (set `self.Timer` _returnvalue)
  (`SceneComponent.SetVisibility` (`self.Sphere`) true false))

(fn `Deactivate`
  (`/Game/Blueprints/DamageSystem/BPI_Damageable.RemoveShield` (`self.Damageable Owner`))
  (`self.K2_DestroyActor`))

(fn `GetShieldCooldownPercent`
  (returns (ShieldPercent :type "Float (double-precision)"))
  (bind _defaultactivetime (`self.DefaultActiveTime`))
  (return (`KismetMathLibrary.SelectFloat` (/ (`KismetSystemLibrary.K2_GetTimerElapsedTimeHandle` (`self.Timer`)) _defaultactivetime) (/ _defaultactivetime _defaultactivetime) (`KismetSystemLibrary.K2_IsTimerActiveHandle` (`self.Timer`)))))

(fn `ReduceCooldown`
  (bind _returnvalue (`KismetSystemLibrary.K2_SetTimer` null "Deactivate" (- (`KismetSystemLibrary.K2_GetTimerRemainingTimeHandle` (`self.Timer`)) 1.0)))
  (set `self.Timer` _returnvalue))

(fn `UserConstructionScript`)