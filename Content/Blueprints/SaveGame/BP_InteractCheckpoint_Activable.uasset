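; Interactable bonfire checkpoint that saves the game through the Game Instance when the player interacts with it.
; The bonfire effects start hidden and are shown by Activate, which Interact calls after requesting the save.
; A sphere overlap shows the interaction widget only while the player pawn is in range.
; The construction script applies light color, radius and intensity variables to the point light, and a debug function toggles the effects.
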(event `self.ReceiveBeginPlay`
  (`self.SetVisibility` false)
  (`self.ChangeTextVisibility` false))

(event `/Game/Blueprints/Interfaces/BPI_Activable.Activate`
  (`self.SetVisibility` true))

(event `/Game/Blueprints/Interfaces/BPI_Interactable.Interact`
  (message `/Game/Blueprints/SaveGame/BPI_SaveGame.SaveGameData` (`GameplayStatics.GetGameInstance`) true)
  (`/Game/Blueprints/Interfaces/BPI_Activable.Activate`))

(event `self.Sphere.OnComponentBeginOverlap`
  (params (OverlappedComponent :type "PrimitiveComponent Object Reference") (OtherActor :type "Actor Object Reference") (OtherComp :type "PrimitiveComponent Object Reference") (OtherBodyIndex :type Integer) (bFromSweep :type Boolean) (SweepResult :type "HitResult Structure (by ref)"))
  (if (== OtherActor (`GameplayStatics.GetPlayerPawn` 0))
    (`self.ChangeTextVisibility` true)))

(event `self.Sphere.OnComponentEndOverlap`
  (params (OverlappedComponent :type "PrimitiveComponent Object Reference") (OtherActor :type "Actor Object Reference") (OtherComp :type "PrimitiveComponent Object Reference") (OtherBodyIndex :type Integer))
  (if (== OtherActor (`GameplayStatics.GetPlayerPawn` 0))
    (`self.ChangeTextVisibility` false)))

(fn `ChangeTextVisibility`
  (params (bVisible :type Boolean))
  (`SceneComponent.SetVisibility` (`self.InteractionWidget`) bVisible false))

(fn `SetVisibility`
  (params (bNewVisibility :type Boolean))
  (`SceneComponent.SetVisibility` (`self.FXS_Bonfire`) bNewVisibility true))

(fn `ToggleEffectsVisibility(Debug)`
  (`SceneComponent.ToggleVisibility` (`self.FXS_Bonfire`) true))

(fn `UserConstructionScript`
  (`LightComponent.SetLightColor` (`self.PointLight`) (`self.LightColor`) true)
  (`LocalLightComponent.SetAttenuationRadius` (`self.PointLight`) (`self.Radius`))
  (`LightComponent.SetIntensity` (`self.PointLight`) (`self.Intensity`)))