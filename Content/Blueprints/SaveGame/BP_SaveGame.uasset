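; BP_SaveGame is the save game object that holds the saved state of statues, plates managers and persistent spawners.
; Getter functions linearly search per-type struct arrays for the given object and return its saved rotation, completion or defeated flag.
; The statue and plates getters also report a Success flag, while the spawner getter has no explicit not-found return.
; GetGameData returns the object itself, and this file contains no write logic.
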(fn `GetGameData`
  (returns (SaveGameData :type "/Game/Blueprints/SaveGame/BP_SaveGame Object Reference"))
  (return self))

(fn `GetPersistentSpawnerState`
  (params (PersistentSpawner :type "/Game/Blueprints/Enemy/Spawners/Parents/BP_PersistentSpawner Object Reference"))
  (returns (bDefeated :type Boolean))
  (for _array_element (`self.PersistentSpawnerStates`)
    (if (== PersistentSpawner (break `/Game/Blueprints/SaveGame/Structures/S_PersistentSpawnerStates` _array_element))
      (`|ExecutionSequence`
        (:`then_0`
          (return (`.bDefeated_5_76C91A344EB29CA019AEF9855243BF8E` (break `/Game/Blueprints/SaveGame/Structures/S_PersistentSpawnerStates` _array_element))))
        (:`then_1`
          (break))))))

(fn `GetPlatesManagerState`
  (params (PlatesManager :type "/Game/Blueprints/Puzzles/Plates/BP_PlatesManager Object Reference"))
  (returns (bIsComplete :type Boolean) (bSuccess :type Boolean))
  (for _array_element (`self.PlatesManagerStates`)
    (if (== PlatesManager (break `/Game/Blueprints/SaveGame/Structures/S_PlateManagerStates` _array_element))
      (`|ExecutionSequence`
        (:`then_0`
          (return (`.bComplete_6_A6ADC6B24299BB03A7BBA299ECEFAD0A` (break `/Game/Blueprints/SaveGame/Structures/S_PlateManagerStates` _array_element)) true))
        (:`then_1`
          (break)))))
  (return false false))

(fn `GetStatueRotation`
  (params (Satue :type "/Game/Blueprints/Puzzles/Statues/BP_Statue Object Reference"))
  (returns (Rotation :type "Float (double-precision)") (bSuccess :type Boolean))
  (for _array_element (`self.StatueRotations`)
    (if (== Satue (break `/Game/Blueprints/SaveGame/Structures/S_StatueRotations` _array_element))
      (`|ExecutionSequence`
        (:`then_0`
          (return (`.StatueRotation_6_59684DD34BE4A7BEC9649894AC805B37` (break `/Game/Blueprints/SaveGame/Structures/S_StatueRotations` _array_element)) true))
        (:`then_1`
          (break)))))
  (return 0.0 false))