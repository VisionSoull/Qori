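; BP_Statue is a rotatable puzzle statue that the player turns toward a desired yaw, reporting to a StatuesManager when correct.
; On game mode ready it restores saved rotation from game data, falling back to its initial rotation.
; The capsule overlap toggles an interaction prompt, and Interact runs a timeline rotation by a set amount.
; A correct rotation can optionally lock interaction and show a point light configured in the construction script.
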(event `self.ReceiveBeginPlay`
  (bind _asbp_qori_game_mode (cast `/Game/Blueprints/BP_QoriGameMode` (`GameplayStatics.GetGameMode`)))
  (add `/Game/Blueprints/BP_QoriGameMode.OnGameModeReady` _asbp_qori_game_mode (delegate `OnGameModeReady_Event`)))

(event `OnGameModeReady_Event`
  (bind _statue (`self.Statue`))
  (bind (_relativerotation_roll _relativerotation_pitch) (`KismetMathLibrary.BreakRotator` (`SceneComponent.RelativeRotation` _statue)))
  (bind _savegamedata (message `/Game/Blueprints/SaveGame/BPI_SaveGame.GetGameData` (`GameplayStatics.GetGameInstance`)))
  (bind (_rotation _bsuccess) (`/Game/Blueprints/SaveGame/BP_SaveGame.GetStatueRotation` _savegamedata self))
  (bind _returnvalue (`KismetMathLibrary.SelectFloat` _rotation (`self.InitialRotation`) _bsuccess))
  (`SceneComponent.K2_SetRelativeRotation` _statue (`KismetMathLibrary.MakeRotator` _relativerotation_roll _relativerotation_pitch _returnvalue) false false)
  (set `self.CurrentRotation` _returnvalue)
  (`self.CheckRotation`)
  (`SceneComponent.SetVisibility` (`self.InteractionWidget`) false false))

(event `self.Capsule.OnComponentBeginOverlap`
  (params (OverlappedComponent :type "PrimitiveComponent Object Reference") (OtherActor :type "Actor Object Reference") (OtherComp :type "PrimitiveComponent Object Reference") (OtherBodyIndex :type Integer) (bFromSweep :type Boolean) (SweepResult :type "HitResult Structure (by ref)"))
  (if (== OtherActor (`GameplayStatics.GetPlayerPawn` 0))
    (`self.ChangeTextVisibility` true)))

(event `self.Capsule.OnComponentEndOverlap`
  (params (OverlappedComponent :type "PrimitiveComponent Object Reference") (OtherActor :type "Actor Object Reference") (OtherComp :type "PrimitiveComponent Object Reference") (OtherBodyIndex :type Integer))
  (if (== OtherActor (`GameplayStatics.GetPlayerPawn` 0))
    (`self.ChangeTextVisibility` false)))

(event `/Game/Blueprints/Interfaces/BPI_Interactable.Interact`
  (bind (_relativerotation_roll _relativerotation_pitch _relativerotation_yaw) (`KismetMathLibrary.BreakRotator` (`SceneComponent.RelativeRotation` (`self.Statue`))))
  ;[0.05098 0.05098 0.05098] Rotate
  (if (`self.bInteractable`)
    (bind _output_get (set `self.InteractInitialRotation` (`SceneComponent.RelativeRotation` (`self.Statue`))))
    (set `self.InteractFinalRotation` (`KismetMathLibrary.MakeRotator` (.roll _output_get) (.pitch _output_get) (+ (.yaw _output_get) (`self.AmountToRotate`))))
    (set `self.bInteractable` false)
    (bind (_direction _time) (`Timeline|TimeToRotate` :!via `PlayFromStart`)
      (:`Update`
        (`SceneComponent.K2_SetRelativeRotation` (`self.Statue`) (`KismetMathLibrary.RLerp` (`self.InteractInitialRotation`) (`self.InteractFinalRotation`) _time) false false))
      (:`Finished`
        (set `self.CurrentRotation` _relativerotation_yaw)
        (`self.CheckRotation`)
        (set `self.bInteractable` true)))))

(fn `ChangeTextVisibility`
  (params (bVisible :type Boolean))
  (`SceneComponent.SetVisibility` (`self.InteractionWidget`) bVisible false))

(fn `CheckRotation`
  (if (== (`self.CurrentRotation`) (`self.DesiredRotation`))
    (set `self.CorrectRotation` true)
    (`/Game/Blueprints/Puzzles/Statues/BP_StatuesManager.CheckCorrectRotations` (`self.StatuesManager`))
    (`|ExecutionSequence`
      (:`then_0`
        (if (`self.bLockWhenCorrect`)
          (`self.SetNotInteractable`)))
      (:`then_1`
        (if (`self.bLightWhenCorrect`)
          (`SceneComponent.SetVisibility` (`self.PointLight`) true false))))
    (else
      (set `self.CorrectRotation` false)
      (`SceneComponent.SetVisibility` (`self.PointLight`) false false))))

(fn `DestroyStatue`
  (`/Game/Blueprints/Puzzles/Statues/BP_StatuesManager.RemoveStatueFromArray` (`self.StatuesManager`) self)
  (`self.K2_DestroyActor`))

(fn `SetNotInteractable`
  (`PrimitiveComponent.SetCollisionEnabled` (`self.Capsule`) "NoCollision")
  (`SceneComponent.SetVisibility` (`self.InteractionWidget`) false false))

(fn `SetStatuesManager`
  (params (StatuesManager :type "/Game/Blueprints/Puzzles/Statues/BP_StatuesManager Object Reference"))
  (set `self.StatuesManager` StatuesManager))

(fn `UserConstructionScript`
  (bind _statue (`self.Statue`))
  (bind (_relativerotation_roll _relativerotation_pitch) (`KismetMathLibrary.BreakRotator` (`SceneComponent.RelativeRotation` _statue)))
  (`LightComponent.SetLightColor` (`self.PointLight`) (`self.LightColor`) true)
  (`LocalLightComponent.SetAttenuationRadius` (`self.PointLight`) (`self.Radius`))
  (`LightComponent.SetIntensity` (`self.PointLight`) (`self.Intensity`))
  (`SceneComponent.K2_SetRelativeRotation` _statue (`KismetMathLibrary.MakeRotator` _relativerotation_roll _relativerotation_pitch (`self.InitialRotation`)) false false))