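; Pressure plate in an ordered plate puzzle, coordinated by a PlatesManager that is passed in.
; When the player pawn overlaps an interactable plate, an active one lights up and asks the manager to activate the next, while an inactive one triggers a puzzle reset.
; Plate number one starts active and stays so on deactivation.
; The plate also exposes functions to lock it lit or remove it from the manager and destroy it.
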(event `self.Collider.OnComponentBeginOverlap`
  (params (OverlappedComponent :type "PrimitiveComponent Object Reference") (OtherActor :type "Actor Object Reference") (OtherComp :type "PrimitiveComponent Object Reference") (OtherBodyIndex :type Integer) (bFromSweep :type Boolean) (SweepResult :type "HitResult Structure (by ref)"))
  (if (== OtherActor (`GameplayStatics.GetPlayerPawn` 0))
    (if (`self.bInteractable`)
      (if (`self.bIsActive`)
        (`self.SetActiveMaterial` true)
        (`/Game/Blueprints/Puzzles/Plates/BP_PlatesManager.SetNextPlateActive` (`self.PlatesManager`) self)
        (else
          (`/Game/Blueprints/Puzzles/Plates/BP_PlatesManager.ResetPlates` (`self.PlatesManager`) true))))))

(fn `Deactivate`
  (`self.SetActiveMaterial` false)
  (set `self.bInteractable` true)
  (if (!= (`self.PlateNumber`) 1)
    (set `self.bIsActive` false)))

(fn `DestroyPlate`
  (`/Game/Blueprints/Puzzles/Plates/BP_PlatesManager.RemovePlateFromArray` (`self.PlatesManager`) self)
  (`self.K2_DestroyActor`))

(fn `SetActive`
  (if (not (`self.bIsActive`))
    (set `self.bIsActive` true)
    (else
      (`/Game/Blueprints/Puzzles/Plates/BP_PlatesManager.ResetPlates` (`self.PlatesManager`) true))))

(fn `SetActiveMaterial`
  (params (bActivated :type Boolean))
  ;[1 1 1] Sets the material corresponding to the plate's active state.
  (if bActivated
    (`PrimitiveComponent.SetMaterial` (`self.Plate`) 1 (`self.MaterialActive`))
    (else
      (`PrimitiveComponent.SetMaterial` (`self.Plate`) 1 (`self.MaterialNormal`)))))

(fn `SetNotInteractable`
  (set `self.bIsActive` true)
  (`self.SetActiveMaterial` true)
  (set `self.bInteractable` false))

(fn `SetNumber`
  (params (Number :type Integer))
  (bind _output_get (set `self.PlateNumber` Number))
  ;[1 1 1] If the plate number is one, it means that it is the first one in the puzzle and Is Active.
  (if (== _output_get 1)
    (set `self.bIsActive` true)
    (else
      (set `self.bIsActive` false))))

(fn `SetPlatesManager`
  (params (PlatesManager :type "/Game/Blueprints/Puzzles/Plates/BP_PlatesManager Object Reference"))
  (set `self.PlatesManager` PlatesManager))

(fn `UserConstructionScript`)