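; Manager for a sequential plate puzzle that numbers its plates by array order and activates actors when the last plate is reached.
; Plates call back to set the next one active; completion locks all plates, triggers the BPI_Activable targets and can reset after a delay.
; Construction and BeginPlay validate both arrays, with helpers to spawn, add or remove plates.
; BeginPlay restores completion from GameInstance game data, falling back to IsComplete if unavailable.
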(event `self.ReceiveBeginPlay`
  (`self.Verify Plate Numbers` true)
  (`self.VerifyValidActivables`)
  (bind _savegamedata (message `/Game/Blueprints/SaveGame/BPI_SaveGame.GetGameData` (`GameplayStatics.GetGameInstance`)))
  (`/Engine/EditorBlueprintResources/StandardMacros.IsValid` _savegamedata
    (:`Is Valid`
      (bind _biscomplete (`/Game/Blueprints/SaveGame/BP_SaveGame.GetPlatesManagerState` _savegamedata self))
      (if _biscomplete
        (`self.Complete Puzzle` :!label _label)))
    (:`Is Not Valid`
      (if (`self.bIsComplete`)
        (goto _label)))))

(event `ResetAfterComplete`
  (`KismetSystemLibrary.Delay` (`self.ResetDelay`))
  (`self.ResetPlates`))

(fn `AddPlateToArray`
  (params (Plate :type "/Game/Blueprints/Puzzles/Plates/BP_Plate Object Reference"))
  (`KismetArrayLibrary.Array_AddUnique` (`self.AllPlates`) Plate)
  (`self.Verify Plate Numbers` false))

(fn `Complete Puzzle`
  (set `self.bIsComplete` true)
  (for _array_element (`self.AllPlates`)
    (`/Game/Blueprints/Puzzles/Plates/BP_Plate.SetNotInteractable` _array_element))
  (for _array_element_2 (`self.Activables`)
    (message `/Game/Blueprints/Interfaces/BPI_Activable.Activate` _array_element_2)
    (if (`self.bResetAfterComplete`)
      (`self.ResetAfterComplete`))))

(fn `CreateNewPlate`
  (bind _returnvalue (`|SpawnActorFromClass` (`self.PlatesClass`) (`self.GetTransform`) "Undefined" "MultiplyWithRoot" null null))
  (`self.AddPlateToArray` _returnvalue))

(fn `RemovePlateFromArray`
  (params (Plate :type "/Game/Blueprints/Puzzles/Plates/BP_Plate Object Reference"))
  (`KismetArrayLibrary.Array_RemoveItem` (`self.AllPlates`) Plate)
  (`self.Verify Plate Numbers` false))

(fn `ResetPlates`
  (for _array_element (`self.AllPlates`)
    (`/Game/Blueprints/Puzzles/Plates/BP_Plate.Deactivate` _array_element))
  (set `self.bIsComplete` false))

(fn `SetNextPlateActive`
  (params (CurrentPlate :type "/Game/Blueprints/Puzzles/Plates/BP_Plate Object Reference"))
  (bind _returnvalue (`KismetArrayLibrary.Array_Find` (`self.AllPlates`) CurrentPlate))
  ;[0.02604 0 0] Check if it is the last plate of the puzzle
  (if (== (`KismetArrayLibrary.Array_LastIndex` (`self.AllPlates`)) _returnvalue)
    (`self.Complete Puzzle`)
    (else
      (`/Game/Blueprints/Puzzles/Plates/BP_Plate.SetActive` (`|GetArrayItem` (`self.AllPlates`) (+ _returnvalue 1))))))

(fn `UserConstructionScript`
  (`self.Verify Plate Numbers` false)
  (if (not (`KismetArrayLibrary.Array_IsEmpty` (`self.Activables`)))
    (for (_array_element _array_index) (`self.Activables`)
      (`/Engine/EditorBlueprintResources/StandardMacros.IsValid` _array_element
        (:`Is Valid`
          (cast `/Game/Blueprints/Interfaces/BPI_Activable` _array_element
            (:`CastFailed`
              (`KismetArrayLibrary.Array_Set` (`self.Activables`) _array_index))))))))

(fn `Verify Plate Numbers`
  (params (bRemoveInvalidElements :type Boolean))
  (bind _allplates (`self.AllPlates`))
  ;[1 1 1] Verify if there are empty indexes in the array and remove them
  (for (_array_element _array_index) (`self.AllPlates`)
    (`/Engine/EditorBlueprintResources/StandardMacros.IsValid` _array_element
      (:`Is Valid`
        (`/Game/Blueprints/Puzzles/Plates/BP_Plate.SetPlatesManager` _array_element self))
      (:`Is Not Valid`
        (if (`local.bRemoveInvalidElements`)
          (`KismetArrayLibrary.Array_Remove` _allplates _array_index)
          (else
            (`KismetArrayLibrary.Array_Set` _allplates _array_index))))))
  ;[1 1 1] Give the plates their respective number
  (for (_array_element_2 _array_index_2) (`self.AllPlates`)
    (`/Game/Blueprints/Puzzles/Plates/BP_Plate.SetNumber` _array_element_2 (+ _array_index_2 1))))

(fn `VerifyValidActivables`
  (for (_array_element _array_index) (`self.Activables`)
    (cast `/Game/Blueprints/Interfaces/BPI_Activable` _array_element
      (:`CastFailed`
        (`KismetArrayLibrary.Array_Remove` (`self.Activables`) _array_index)))))