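; AIC_Enemy is an AI controller that keeps a BP_AIEnemy pawn leashed to its InitialSpot actor.
; On BeginPlay it caches the controlled pawn, places it at that spot and passes the spot's location to the pawn's LookAtMessage.
; Every Tick it checks the pawn's distance to the spot and, beyond a fixed radius, sends it back through a MoveTo wrapper around MoveToActor.
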(event `self.ReceiveTick`
  (params (DeltaSeconds :type "Float (single-precision)"))
  (bind _stores_pawn (`self.Stores Pawn`))
  (bind _initialspot (`/Game/Blueprints/BasicAI/BP_AIEnemy.InitialSpot` _stores_pawn))
  (if (> (`self.GetDistanceTo` _stores_pawn _initialspot) 500.0)
    (`self.MoveTo` _initialspot)))

(event `self.ReceiveBeginPlay`
  (bind _asbp_aienemy (cast `/Game/Blueprints/BasicAI/BP_AIEnemy` (`self.K2_GetPawn`)))
  (bind _output_get (set `self.Stores Pawn` _asbp_aienemy))
  (bind _returnvalue (`self.K2_GetActorLocation` (`/Game/Blueprints/BasicAI/BP_AIEnemy.InitialSpot` _output_get)))
  (`self.K2_SetActorLocation` _output_get _returnvalue false false)
  (message `/Game/Blueprints/Interfaces/BPI_Character.LookAt` _output_get _returnvalue))

(fn `MoveTo`
  (params (TargetToMoveTo :type "Actor Object Reference"))
  (`self.MoveToActor` TargetToMoveTo -1.0 true true true null))

(fn `UserConstructionScript`)