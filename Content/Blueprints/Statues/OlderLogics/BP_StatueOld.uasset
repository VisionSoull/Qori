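; BP_StatueOld is a rotatable puzzle statue that shows a text prompt while the player overlaps its capsule.
; Interact turns the mesh by a set yaw step through a timeline lerp, blocking further input until it finishes.
; It then compares yaw to the desired value by exact equality, notifying StatuesManager on a match; construction runs the same check.
; SetNotInteractable permanently disables it by destroying the capsule and hiding the prompt.
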(event `self.Capsule.OnComponentBeginOverlap`
  (params (OverlappedComponent :type "PrimitiveComponent Object Reference") (OtherActor :type "Actor Object Reference") (OtherComp :type "PrimitiveComponent Object Reference") (OtherBodyIndex :type Integer) (bFromSweep :type Boolean) (SweepResult :type "HitResult Structure (by ref)"))
  (if (== OtherActor (`GameplayStatics.GetPlayerPawn` 0))
    (if (`self.bInteractable`)
      (`self.ChangeVisibility` true))))

(event `self.Capsule.OnComponentEndOverlap`
  (params (OverlappedComponent :type "PrimitiveComponent Object Reference") (OtherActor :type "Actor Object Reference") (OtherComp :type "PrimitiveComponent Object Reference") (OtherBodyIndex :type Integer))
  (if (== OtherActor (`GameplayStatics.GetPlayerPawn` 0))
    (`self.ChangeVisibility` false)))

(event `self.Interact`
  (bind (_relativerotation_roll _relativerotation_pitch _relativerotation_yaw) (`KismetMathLibrary.BreakRotator` (`SceneComponent.RelativeRotation` (`self.Statue`))))
  ;[0.05098 0.05098 0.05098] Rotate
  (if (`self.bInteractable`)
    (bind _output_get (set `self.InteractInitialRotation` (`SceneComponent.RelativeRotation` (`self.Statue`))))
    (set `self.InteractFinalRotation` (`KismetMathLibrary.MakeRotator` (.roll _output_get) (.pitch _output_get) (+ (.yaw _output_get) (`self.AmountToRotate`))))
    (set `self.bInteractable` false)
    (bind (_direction _time) (`Timeline|TimeToRotate` :!via `PlayFromStart`)
      (:`Update`
        (`SceneComponent.K2_SetRelativeRotation` (`self.Statue`) (`KismetMathLibrary.RLerp` (`self.InteractInitialRotation`) (`self.InteractFinalRotation`) _time) false false))
      (:`Finished`
        (set `self.CurrentRotation` _relativerotation_yaw)
        (`self.CheckRotation`)
        (set `self.bInteractable` true)))))

(fn `ChangeVisibility`
  (params (bVisible :type Boolean))
  (`SceneComponent.SetVisibility` (`self.TextRender`) bVisible false))

(fn `CheckRotation`
  (if (== (`self.CurrentRotation`) (`self.DesiredRotation`))
    (set `self.CorrectRotation` true)
    (`KismetSystemLibrary.PrintString` "Correct Rotation")
    (`/Game/Blueprints/Statues/OlderLogics/BP_StatuesManagerOld.CheckCorrectRotations` (`self.StatuesManager`))
    (else
      (set `self.CorrectRotation` false))))

(fn `SetNotInteractable`
  (`ActorComponent.K2_DestroyComponent` (`self.Capsule`))
  (set `self.bInteractable` false)
  (`self.ChangeVisibility` false))

(fn `SetStatuesManager`
  (params (Statuesmanager :type "/Game/Blueprints/Statues/OlderLogics/BP_StatuesManagerOld Object Reference"))
  (set `self.StatuesManager` Statuesmanager))

(fn `UserConstructionScript`
  (bind _statue (`self.Statue`))
  (bind (_relativerotation_roll _relativerotation_pitch _relativerotation_yaw) (`KismetMathLibrary.BreakRotator` (`SceneComponent.RelativeRotation` _statue)))
  (`SceneComponent.SetVisibility` (`self.TextRender`) (`self.bTextVisible`) false)
  (`SceneComponent.K2_SetRelativeRotation` _statue (`KismetMathLibrary.MakeRotator` _relativerotation_roll _relativerotation_pitch (`self.InitialRotation`)) false false)
  (set `self.CurrentRotation` _relativerotation_yaw)
  (`self.CheckRotation`)
  (set `self.bInteractable` true))