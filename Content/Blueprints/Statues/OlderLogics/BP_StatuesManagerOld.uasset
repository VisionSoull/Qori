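; Statue puzzle manager that activates a linked object once every statue in its list has the correct rotation.
; The construction script registers the manager on each statue and checks that the linked Activable implements BPI_Activable, printing the result and clearing invalid references.
; CheckCorrectRotations stops at the first wrong statue, otherwise CompletePuzzle makes all statues non-interactable and sends ActivateMessage to the Activable.
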(fn `CheckCorrectRotations`
  (for _array_element (`self.AllStatues`)
    (if (`/Game/Blueprints/Statues/OlderLogics/BP_StatueOld.CorrectRotation` _array_element)
      (set `self.bStatuesComplete` true)
      (else
        (set `self.bStatuesComplete` false)
        (break))))
  (if (`self.bStatuesComplete`)
    (`self.CompletePuzzle`)))

(fn `CompletePuzzle`
  (for _array_element (`self.AllStatues`)
    (`/Game/Blueprints/Statues/OlderLogics/BP_StatueOld.SetNotInteractable` _array_element))
  (message `/Game/Blueprints/Interfaces/BPI_Activable.Activate` (`self.Activable`)))

(fn `UserConstructionScript`
  (bind _activable (`self.Activable`))
  (bind _returnvalue (`KismetSystemLibrary.GetDisplayName` _activable))
  (for _array_element (`self.AllStatues`)
    (`/Game/Blueprints/Statues/OlderLogics/BP_StatueOld.SetStatuesManager` _array_element self)
    (`/Engine/EditorBlueprintResources/StandardMacros.IsValid` _activable
      (:`Is Valid`
        (cast `/Game/Blueprints/Interfaces/BPI_Activable` _activable
          (:`then`
            (`/Engine/EditorBlueprintResources/StandardMacros.DoOnce` false
              (:`Completed`
                (`KismetSystemLibrary.PrintString` (`KismetStringLibrary.Concat_StrStr` _returnvalue ":: Inherits Activable Interface") true true (struct :`G` 0.66 :`B` 1.0 :`A` 1.0) 20.0))))
          (:`CastFailed`
            (`KismetSystemLibrary.PrintString` (`KismetStringLibrary.Concat_StrStr` _returnvalue ":: Does not Inherit from Activable Interface") true true (struct :`R` 1.0 :`A` 1.0) 20.0)
            (set `self.Activable` null)))))))