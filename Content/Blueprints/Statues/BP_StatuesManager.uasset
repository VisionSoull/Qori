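; Manager actor for a statue rotation puzzle that activates linked actors once every registered statue has the correct rotation.
; It spawns or registers statues with a back-reference to itself, and CheckCorrectRotations completes the puzzle, locking statues and sending ActivateMessage to Activables.
; Construction and BeginPlay prune invalid statues, draw debug lines to the rest, and flag and clear Activables lacking BPI_Activable with on-screen warnings.
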(event `self.ReceiveBeginPlay`
  (`self.VerifyStatues`)
  (`self.VerifyValidActivables`))

(fn `AddStatueToArray`
  (params (Statue :type "/Game/Blueprints/Statues/BP_Statue Object Reference"))
  (`KismetArrayLibrary.Array_AddUnique` (`self.AllStatues`) Statue)
  (`/Game/Blueprints/Statues/BP_Statue.SetStatuesManager` Statue self))

(fn `CeateNewStatue`
  (bind _returnvalue (`|SpawnActorFromClass` (`self.StatueClass`) (`self.GetTransform`) "Undefined" "MultiplyWithRoot" null null))
  (`self.AddStatueToArray` _returnvalue))

(fn `CheckCorrectRotations`
  (for _array_element (`self.AllStatues`)
    (if (`/Game/Blueprints/Statues/BP_Statue.CorrectRotation` _array_element)
      (set `self.bStatuesComplete` true)
      (else
        (set `self.bStatuesComplete` false)
        (break))))
  (if (`self.bStatuesComplete`)
    (`self.CompletePuzzle`)))

(fn `CompletePuzzle`
  (for _array_element (`self.AllStatues`)
    (`/Game/Blueprints/Statues/BP_Statue.SetNotInteractable` _array_element))
  (for _array_element_2 (`self.Activables`)
    (message `/Game/Blueprints/Interfaces/BPI_Activable.Activate` _array_element_2)))

(fn `DrawDebugLines`
  (`KismetSystemLibrary.FlushPersistentDebugLines`)
  (for _array_element (`self.AllStatues`)
    (`KismetSystemLibrary.DrawDebugLine` (`self.K2_GetActorLocation` self) (`self.K2_GetActorLocation` _array_element) (struct :`R` 1.0 :`B` 0.940621 :`A` 1.0) 5.0))
  (return))

(fn `RemoveStatueFromArray`
  (params (Statue :type "/Game/Blueprints/Statues/BP_Statue Object Reference"))
  (`KismetArrayLibrary.Array_RemoveItem` (`self.AllStatues`) Statue)
  (`self.VerifyStatues`))

(fn `UserConstructionScript`
  (`self.VerifyStatues`)
  (if (not (`KismetArrayLibrary.Array_IsEmpty` (`self.Activables`)))
    (for (_array_element _array_index) (`self.Activables`)
      (`/Engine/EditorBlueprintResources/StandardMacros.IsValid` _array_element
        (:`Is Valid`
          (cast `/Game/Blueprints/Interfaces/BPI_Activable` _array_element
            (:`CastFailed`
              (`KismetSystemLibrary.PrintString` (`KismetStringLibrary.Concat_StrStr` (`KismetSystemLibrary.GetDisplayName` _array_element) ":: Does not Inherit from Activable Interface") true true (struct :`R` 1.0 :`A` 1.0) 10.0)
              (`KismetArrayLibrary.Array_Set` (`self.Activables`) _array_index))))))))

(fn `VerifyStatues`
  ;[1 1 1] Verify if there are empty indexes in the array and remove them
  (for (_array_element _array_index) (`self.AllStatues`)
    (`/Engine/EditorBlueprintResources/StandardMacros.IsValid` _array_element
      (:`Is Not Valid`
        (`KismetArrayLibrary.Array_Remove` (`self.AllStatues`) _array_index))))
  ;[1 0.8569 0] Debug
  (`self.DrawDebugLines`))

(fn `VerifyValidActivables`
  (for (_array_element _array_index) (`self.Activables`)
    (cast `/Game/Blueprints/Interfaces/BPI_Activable` _array_element
      (:`then`
        (`/Engine/EditorBlueprintResources/StandardMacros.DoOnce` false
          (:`Completed`
            (bind _returnvalue (`KismetSystemLibrary.GetDisplayName` _array_element))
            (`KismetSystemLibrary.PrintString` (`KismetStringLibrary.Concat_StrStr` _returnvalue ":: Inherits Activable Interface") true true (struct :`G` 0.66 :`B` 1.0 :`A` 1.0) 20.0))))
      (:`CastFailed`
        (`KismetSystemLibrary.PrintString` (`KismetStringLibrary.Concat_StrStr` _returnvalue ":: Does not Inherit from Activable Interface") true true (struct :`R` 1.0 :`A` 1.0) 20.0)
        (`KismetArrayLibrary.Array_Remove` (`self.Activables`) _array_index)))))