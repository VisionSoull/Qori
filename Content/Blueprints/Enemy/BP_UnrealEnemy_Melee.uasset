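; BP_UnrealEnemy_Melee is a melee enemy Blueprint that equips BP_Sword as its weapon and attacks with a sword slash.
; Attack calls the parent, then plays a slowed slash montage, tracking IsAttacking until it completes or is interrupted.
; Montage notify begin and end toggle the weapon's attacking state.
; When the montage ends, CallOnAttackEnd signals a Behavior Tree task that the attack is over.
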(event `self.Attack`
  (bind _weaponobject (`self.WeaponObject`))
  (`parent.Attack`)
  (bind _notifyname (`|PlayMontage` (`self.Mesh`) "/Game/Characters/Animations/Melee/AM_SwordSlash.AM_SwordSlash" 0.7)
    (:`then`
      (set `self.bIsAttacking` true))
    (:`OnCompleted`
      (set `self.bIsAttacking` false :!label _label)
      (`self.OnAttackEnd`) ; Subscriber on Behavior Tree Task
    )
    (:`OnInterrupted`
      (goto _label))
    (:`OnNotifyBegin`
      (switch `name` _notifyname
        (:`Slash`
          (`/Game/Blueprints/Weapons/BP_Weapon.IsAttacking` _weaponobject true))))
    (:`OnNotifyEnd`
      (switch `name` _notifyname
        (:`Slash`
          (`/Game/Blueprints/Weapons/BP_Weapon.IsAttacking` _weaponobject false))))))

(fn `UserConstructionScript`
  (`parent.UserConstructionScript`)
  (set `self.Weapon` "/Game/Blueprints/Weapons/BP_Sword.BP_Sword_C"))