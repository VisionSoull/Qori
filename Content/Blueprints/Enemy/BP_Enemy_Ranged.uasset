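; BP_Enemy_Ranged is a ranged enemy that carries a spear and attacks by launching a projectile at its focus target.
; Attack plays a montage, whose notify hides the weapon and spawns a projectile aimed from it at the AI controller's focus actor, passing on wielder and damage.
; Montage completion or interruption restores the weapon, clears the attacking flag and signals attack end.
; GetIdealRange supplies its preferred distance from the target.
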(event `self.Attack`
  (bind _returnvalue (`self.K2_GetActorLocation` (`self.WeaponObject`)))
  (`parent.Attack`)
  (bind _notifyname (`|PlayMontage` (`self.Mesh`) (`self.AttackMontage`) 1.5)
    (:`then`
      (set `self.bIsAttacking` true))
    (:`OnCompleted`
      (set `self.bIsAttacking` false :!label _label)
      (`/Game/Blueprints/Weapons/BP_Weapon.SetVisibility` (`self.WeaponObject`) true)
      (`self.OnAttackEnd`))
    (:`OnInterrupted`
      (goto _label))
    (:`OnNotifyBegin`
      (switch `name` _notifyname
        (:`SendProjectile`
          (`/Game/Blueprints/Weapons/BP_Weapon.SetVisibility` (`self.WeaponObject`) false)
          (bind _returnvalue_2 (`|SpawnActorFromClass` (`self.Projectile`) (`KismetMathLibrary.MakeTransform` _returnvalue (`KismetMathLibrary.FindLookAtRotation` _returnvalue (`self.K2_GetActorLocation` (`AIController.GetFocusActor` (`self.AICEnemyBase`))))) "AlwaysSpawn" "MultiplyWithRoot" self null))
          (`/Game/Blueprints/Weapons/BP_Projectile.Setup Projectile` _returnvalue_2 self (`self.AttackDamageAmount`)))))))

(fn `GetIdealRange`
  (returns (IdealRange :type "Float (double-precision)"))
  (return (`self.IdealRangeFromTarget`)))

(fn `UserConstructionScript`
  (`parent.UserConstructionScript`)
  (set `self.Weapon` "/Game/Blueprints/Weapons/BP_Spear.BP_Spear_C"))