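; Parent enemy spawner that stays empty after loading a save in which its enemy was defeated.
; BeginPlay reads its Defeated state through the GameInstance, spawning when undefeated or no data exists.
; Spawn sphere-traces down the resizable box for static floor or BP_FloorGrid, then spawns EnemyToSpawn with its class-default Behavior Tree and random yaw.
; The enemy's OnDeath sets Defeated, which comments say is saved at checkpoints.
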(event `self.ReceiveBeginPlay`
  ;[0.1406 0 0.01459] Begin Play
  (bind _bexists (message `/Game/Blueprints/SaveGame/BPI_SaveGame.DoesSaveGameExist` (`GameplayStatics.GetGameInstance`)))
  (if _bexists
    (bind _savegamedata (message `/Game/Blueprints/SaveGame/BPI_SaveGame.GetGameData` (`GameplayStatics.GetGameInstance`)))
    (bind (_bdefeated _bsuccess) (`/Game/Blueprints/SaveGame/BP_SaveGame.GetPersistentSpawnerState` _savegamedata self)) ; Get Data from Save Game to determine if it spawns \nusing the Save's variable or spawn if it wasn't possible\nto optain the Data
    (if _bsuccess
      (bind _output_get (set `self.bDefeated` _bdefeated))
      (if (not _output_get)
        (`self.Spawn`))
      (else
        (`self.Spawn`)))
    (else
      (set `self.bDefeated` false)
      (`self.Spawn`))))

(event `Spawn`
  (bind (_returnvalue_roll _returnvalue_pitch _returnvalue_yaw) (`KismetMathLibrary.BreakRotator` (`KismetMathLibrary.RandomRotator` false)))
  (bind _enemytospawn (`self.EnemyToSpawn`))
  (bind (_origin _boxextent) (`KismetSystemLibrary.GetComponentBounds` (`self.Box`)))
  (bind _z (.z _boxextent))
  (bind _z_2 (.z _origin))
  (bind _returnvalue (`KismetMathLibrary.MakeVector` (.x _origin) (.y _origin) (+ _z_2 _z)))
  ;[0.1094 0.09633 0] Spawn
  (`/Engine/EditorBlueprintResources/StandardMacros.IsValid` (`self.SpawnedAI`)
    (:`Is Not Valid`
      (bind (_outhit _returnvalue_2) (`KismetSystemLibrary.SphereTraceSingleForObjects` :`Start` _returnvalue :`End` (`KismetMathLibrary.MakeVector` (.x _returnvalue) (.y _returnvalue) (- _z_2 _z)) :`Radius` 40.0 :`ObjectTypes` (`|MakeArray` "ObjectTypeQuery3" "ObjectTypeQuery1" "ObjectTypeQuery2" :!type "EObjectTypeQuery Enum") :`bTraceComplex` true :`DrawTime` 1.0)) ; Makes a sphere trace from the top of the Box Collider to the bottom \nto detect a floor to spawn the enemy.
      (if _returnvalue_2
        (bind (_bblockinghit _binitialoverlap _time _distance _location _impactpoint _normal _impactnormal _physmat _hitactor _hitcomponent) (`GameplayStatics.BreakHitResult` _outhit))
        (switch `ECollisionChannel` (`PrimitiveComponent.GetCollisionObjectType` _hitcomponent)
          (:`ECC_WorldStatic`
            (bind _returnvalue_3 (`AIBlueprintHelperLibrary.SpawnAIFromClass` _enemytospawn (`.BehaviorTree` (defaults `Object` _enemytospawn)) _location (`KismetMathLibrary.MakeRotator` 0.0 0.0 _returnvalue_yaw) false null :!label _label))
            (bind _output_get (set `self.SpawnedAI` _returnvalue_3))
            (set `self.bDefeated` false)
            (bind _asbp_enemy_base (cast `/Game/Blueprints/Enemy/BP_Enemy_Base` _output_get))
            (add `/Game/Blueprints/Enemy/BP_Enemy_Base.OnDeath` _asbp_enemy_base (delegate `SetDefeated`)) ; When this enemy is defeated the bDefeated variables is set to \ntrue in order to Save this Data when a Checkpoint is crossed
          )
          (:`ECC_WorldDynamic`
            (if (== (`GameplayStatics.GetObjectClass` _hitactor) "/Game/Blueprints/Environment/BP_FloorGrid.BP_FloorGrid_C")
              (goto _label))))))))

(event `SetDefeated`
  ;[0.1094 0.09633 0] Spawn
  (set `self.bDefeated` true))

(fn `UserConstructionScript`
  (bind _extentz (`self.ExtentZ`))
  (`BoxComponent.SetBoxExtent` (`self.Box`) (`KismetMathLibrary.MakeVector` (`self.ExtentX`) (`self.ExtentY`) _extentz) true)
  (`SceneComponent.K2_SetRelativeLocation` (`self.Box`) (`KismetMathLibrary.MakeVector` 0.0 0.0 _extentz) false false))