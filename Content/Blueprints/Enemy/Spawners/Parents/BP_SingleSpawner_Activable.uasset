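; Single-enemy spawner that, when activated, spawns one AI if none is alive and triggers its linked Activables when that enemy dies.
; A sphere trace down the box center must hit BP_FloorGrid; the enemy spawns there with random yaw, retrying failed spawns up to an attempt limit.
; The construction script sizes the box and registers itself with linked BPI_Activable actors.
; BeginPlay prunes invalid links and can auto-activate for debugging.
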(event `self.ReceiveBeginPlay`
  (`self.VerifyValidActivables`)
  (if (`self.OnBeginPlay(Debug)`)
    (`self.Activate`)))

(event `/Game/Blueprints/Interfaces/BPI_Activable.Activate`
  (bind (_returnvalue_roll _returnvalue_pitch _returnvalue_yaw) (`KismetMathLibrary.BreakRotator` (`KismetMathLibrary.RandomRotator` false)))
  (bind _enemytospawn (`self.EnemyToSpawn`))
  (bind (_origin _boxextent) (`KismetSystemLibrary.GetComponentBounds` (`self.Box`)))
  (bind _z (.z _origin))
  (bind _z_2 (.z _boxextent))
  (bind _returnvalue (`KismetMathLibrary.MakeVector` (.x _origin) (.y _origin) (+ _z _z_2)))
  (`/Engine/EditorBlueprintResources/StandardMacros.IsValid` (`self.SpawnedAI`)
    (:`Is Not Valid`
      (if (< (`self.SpawnAttemps`) (`self.MaximumAttempts`)) :!label _label
        (bind (_outhit _returnvalue_2) (`KismetSystemLibrary.SphereTraceSingleForObjects` :`Start` _returnvalue :`End` (`KismetMathLibrary.MakeVector` (.x _returnvalue) (.y _returnvalue) (- _z _z_2)) :`Radius` 40.0 :`ObjectTypes` (`|MakeArray` "ObjectTypeQuery3" "ObjectTypeQuery1" "ObjectTypeQuery2" :!type "EObjectTypeQuery Enum") :`bTraceComplex` true :`DrawTime` 1.0))
        (if _returnvalue_2
          (bind (_bblockinghit _binitialoverlap _time _distance _location _impactpoint _normal _impactnormal _physmat _hitactor _hitcomponent) (`GameplayStatics.BreakHitResult` _outhit))
          (switch `ECollisionChannel` (`PrimitiveComponent.GetCollisionObjectType` _hitcomponent)
            (:`ECC_WorldStatic`
              _)
            (:`ECC_WorldDynamic`
              _))
          (if (== (`GameplayStatics.GetObjectClass` _hitactor) "/Game/Blueprints/Environment/BP_FloorGrid.BP_FloorGrid_C")
            (bind _returnvalue_3 (`AIBlueprintHelperLibrary.SpawnAIFromClass` _enemytospawn (`.BehaviorTree` (defaults `Object` _enemytospawn)) _location (`KismetMathLibrary.MakeRotator` 0.0 0.0 _returnvalue_yaw) false null))
            (bind (_asbp_enemy_base _bsuccess) (cast `/Game/Blueprints/Enemy/BP_Enemy_Base` _returnvalue_3 :!pure true))
            (if _bsuccess
              (bind _output_get (set `self.SpawnedAI` _asbp_enemy_base))
              (bind _asbp_enemy_base_2 (cast `/Game/Blueprints/Enemy/BP_Enemy_Base` _output_get))
              (add `/Game/Blueprints/Enemy/BP_Enemy_Base.OnDeath` _asbp_enemy_base_2 (delegate `SpawnedAIDefeated`))
              (else
                (`/Engine/EditorBlueprintResources/StandardMacros.IncrementInt` (`self.SpawnAttemps`)
                  (:`  `
                    (goto _label)))))))))))

(event `SpawnedAIDefeated`
  (set `self.SpawnedAI` null)
  (for _array_element (`self.Activables`)
    (message `/Game/Blueprints/Interfaces/BPI_Activable.Activate` _array_element)))

(fn `UserConstructionScript`
  (bind _extentz (`self.ExtentZ`))
  (`BoxComponent.SetBoxExtent` (`self.Box`) (`KismetMathLibrary.MakeVector` (`self.ExtentX`) (`self.ExtentY`) _extentz) true)
  (`SceneComponent.K2_SetRelativeLocation` (`self.Box`) (`KismetMathLibrary.MakeVector` 0.0 0.0 _extentz) false false)
  (for (_array_element _array_index) (`self.Activables`)
    (`/Engine/EditorBlueprintResources/StandardMacros.IsValid` _array_element
      (:`Is Valid`
        (cast `/Game/Blueprints/Interfaces/BPI_Activable` _array_element
          (:`then`
            (message `/Game/Blueprints/Interfaces/BPI_ActivableIntermediary.AddConnectorToList` _array_element self))
          (:`CastFailed`
            (`KismetArrayLibrary.Array_Set` (`self.Activables`) _array_index)))))))

(fn `VerifyValidActivables`
  (for (_array_element _array_index) (`self.Activables`)
    (cast `/Game/Blueprints/Interfaces/BPI_Activable` _array_element
      (:`CastFailed`
        (`KismetArrayLibrary.Array_Remove` (`self.Activables`) _array_index)))))