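; Area spawner that, once activated, spawns a set number of random enemy types inside an editor-sized box, with a delay between spawns.
; Downward sphere traces at random box points pick spawn locations, and failed spawns retry up to an attempt limit.
; Enemy deaths update counters and the game mode's task display.
; When the live count reaches zero, it triggers linked BPI_Activable actors, which register it as a connector during construction.
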(event `self.ReceiveBeginPlay`
  (set `self.EnemiesSpawned` 0)
  (set `self.EnemiesDefeated` 0)
  (`self.VerifyValidActivables`)
  (if (`self.OnBeginPlay(Debug)`)
    (`self.Activate`)))

(event `/Game/Blueprints/Interfaces/BPI_Activable.Activate`
  (bind (_returnvalue_roll _returnvalue_pitch _returnvalue_yaw) (`KismetMathLibrary.BreakRotator` (`KismetMathLibrary.RandomRotator` false)))
  (bind _outitem (`KismetArrayLibrary.Array_Random` (`self.EnemyToSpawn`)))
  (bind (_origin _boxextent) (`KismetSystemLibrary.GetComponentBounds` (`self.Box`)))
  (bind _z (.z _boxextent))
  (bind _z_2 (.z _origin))
  (bind (_returnvalue_x _returnvalue_y) (`KismetMathLibrary.BreakVector` (`KismetMathLibrary.RandomPointInBoundingBox` _origin _boxextent)))
  (bind _returnvalue (`KismetMathLibrary.MakeVector` _returnvalue_x _returnvalue_y (+ _z_2 _z)))
  (if (< (`self.EnemiesSpawned`) (`self.NumberOfEnemiesToSpawn`))
    (if (not (== (`self.EnemiesSpawned`) 0))
      (`KismetSystemLibrary.Delay` (`self.TimerBetweenSpawnsInSeconds`)))
    (if (< (`self.SpawnAttemps`) (`self.MaximumAttempts`))
      (bind (_outhit _returnvalue_2) (`KismetSystemLibrary.SphereTraceSingleForObjects` :`Start` _returnvalue :`End` (`KismetMathLibrary.MakeVector` (.x _returnvalue) (.y _returnvalue) (- _z_2 _z)) :`Radius` 40.0 :`ObjectTypes` (`|MakeArray` "ObjectTypeQuery1" "ObjectTypeQuery2" :!type "EObjectTypeQuery Enum") :`DrawTime` 1.0))
      (if _returnvalue_2
        (bind (_bblockinghit _binitialoverlap _time _distance _location _impactpoint _normal _impactnormal _physmat _hitactor _hitcomponent) (`GameplayStatics.BreakHitResult` _outhit))
        (switch `ECollisionChannel` (`PrimitiveComponent.GetCollisionObjectType` _hitcomponent)
          (:`ECC_WorldStatic`
            _)
          (:`ECC_WorldDynamic`
            _))
        (bind _returnvalue_3 (`AIBlueprintHelperLibrary.SpawnAIFromClass` _outitem (`.BehaviorTree` (defaults `Object` _outitem)) _location (`KismetMathLibrary.MakeRotator` 0.0 0.0 _returnvalue_yaw) false null))
        (bind (_asbp_enemy_base _bsuccess) (cast `/Game/Blueprints/Enemy/BP_Enemy_Base` _returnvalue_3 :!pure true))
        (if _bsuccess
          (`KismetArrayLibrary.Array_AddUnique` (`self.SpawnedAI`) _asbp_enemy_base)
          (add `/Game/Blueprints/Enemy/BP_Enemy_Base.OnDeath` _asbp_enemy_base (delegate `RemoveSpawnedAI`))
          (`/Engine/EditorBlueprintResources/StandardMacros.IncrementInt` (`self.EnemiesSpawned`)
            (:`  `
              (`/Game/Blueprints/Interfaces/BPI_Activable.Activate`)))
          (else
            (`/Engine/EditorBlueprintResources/StandardMacros.IncrementInt` (`self.SpawnAttemps`)
              (:`  `
                (`/Game/Blueprints/Interfaces/BPI_Activable.Activate`)))))))))

(event `RemoveSpawnedAI`
  (bind _returnvalue (`GameplayStatics.GetGameMode`))
  (bind _numberofenemiestospawn (`self.NumberOfEnemiesToSpawn`))
  (bind _result (`/Engine/EditorBlueprintResources/StandardMacros.IncrementInt` (`self.EnemiesDefeated`))
    (:`  `
      (if (== _result _numberofenemiestospawn)
        (set `self.EnemiesDefeated` _numberofenemiestospawn))
      (bind _result_2 (`/Engine/EditorBlueprintResources/StandardMacros.DecrementInt` (`self.EnemiesSpawned`))
        (:`  `
          (if (== _result_2 0)
            (for _array_element (`self.Activables`)
              (message `/Game/Blueprints/Interfaces/BPI_Activable.Activate` _array_element))
            (message `/Game/Blueprints/Interfaces/BPI_TasksHandler.UpdateCurrentTask` _returnvalue self)
            (message `/Game/Blueprints/Interfaces/BPI_TasksHandler.UpdateTaskList` _returnvalue self false)
            (else
              (message `/Game/Blueprints/Interfaces/BPI_TasksHandler.UpdateCurrentTask` (`GameplayStatics.GetGameMode`) self))))))))

(fn `GetCurrentCount`
  (returns (CurrentCount :type Integer))
  (return (`self.EnemiesDefeated`)))

(fn `UserConstructionScript`
  (bind _extentz (`self.ExtentZ`))
  (`BoxComponent.SetBoxExtent` (`self.Box`) (`KismetMathLibrary.MakeVector` (`self.ExtentX`) (`self.ExtentY`) _extentz) true)
  (`SceneComponent.K2_SetRelativeLocation` (`self.Box`) (`KismetMathLibrary.MakeVector` 0.0 0.0 _extentz) false false)
  (for (_array_element _array_index) (`self.Activables`)
    (`/Engine/EditorBlueprintResources/StandardMacros.IsValid` _array_element
      (:`Is Valid`
        (cast `/Game/Blueprints/Interfaces/BPI_Activable` _array_element
          (:`then`
            (message `/Game/Blueprints/Interfaces/BPI_ActivableIntermediary.AddConnectorToList` _array_element self))
          (:`CastFailed`
            (`KismetArrayLibrary.Array_Set` (`self.Activables`) _array_index)))))))

(fn `VerifyValidActivables`
  (for (_array_element _array_index) (`self.Activables`)
    (cast `/Game/Blueprints/Interfaces/BPI_Activable` _array_element
      (:`CastFailed`
        (`KismetArrayLibrary.Array_Remove` (`self.Activables`) _array_index)))))