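; Parent enemy spawner that spawns a single AI enemy, skipping it if the saved game state marks it as defeated.
; BeginPlay reads that state through the GameInstance and activates the spawner when undefeated or unsaved.
; Activation sphere-traces down through the construction-sized box, spawning only on a WorldStatic hit, with random yaw and the enemy class's default behavior tree.
; The enemy's death event sets the Defeated flag.
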(event `self.ReceiveBeginPlay`
  (bind _bexists (message `/Game/Blueprints/SaveGame/BPI_SaveGame.DoesSaveGameExist` (`GameplayStatics.GetGameInstance`)))
  (if _bexists
    (bind _savegamedata (message `/Game/Blueprints/SaveGame/BPI_SaveGame.GetGameData` (`GameplayStatics.GetGameInstance`)))
    (bind _bdefeated (`/Game/Blueprints/SaveGame/BP_SaveGame.GetPersistentSpawnerState` _savegamedata self))
    (bind _output_get (set `self.bDefeated` _bdefeated))
    (if (not _output_get)
      (`/Game/Blueprints/Interfaces/BPI_Activable.Activate`))
    (else
      (set `self.bDefeated` false)
      (`/Game/Blueprints/Interfaces/BPI_Activable.Activate`))))

(event `/Game/Blueprints/Interfaces/BPI_Activable.Activate`
  (bind (_returnvalue_roll _returnvalue_pitch _returnvalue_yaw) (`KismetMathLibrary.BreakRotator` (`KismetMathLibrary.RandomRotator` false)))
  (bind _enemytospawn (`self.EnemyToSpawn`))
  (bind (_origin _boxextent) (`KismetSystemLibrary.GetComponentBounds` (`self.Box`)))
  (bind _z (.z _boxextent))
  (bind _z_2 (.z _origin))
  (bind _returnvalue (`KismetMathLibrary.MakeVector` (.x _origin) (.y _origin) (+ _z_2 _z)))
  (bind (_outhit _returnvalue_2) (`KismetSystemLibrary.SphereTraceSingleForObjects` :`Start` _returnvalue :`End` (`KismetMathLibrary.MakeVector` (.x _returnvalue) (.y _returnvalue) (- _z_2 _z)) :`Radius` 40.0 :`ObjectTypes` (`|MakeArray` "ObjectTypeQuery3" "ObjectTypeQuery1" :!type "EObjectTypeQuery Enum") :`DrawTime` 1.0))
  (if _returnvalue_2
    (bind (_bblockinghit _binitialoverlap _time _distance _location _impactpoint _normal _impactnormal _physmat _hitactor _hitcomponent) (`GameplayStatics.BreakHitResult` _outhit))
    (switch `ECollisionChannel` (`PrimitiveComponent.GetCollisionObjectType` _hitcomponent)
      (:`ECC_WorldStatic`
        (bind _returnvalue_3 (`AIBlueprintHelperLibrary.SpawnAIFromClass` _enemytospawn (`.BehaviorTree` (defaults `Object` _enemytospawn)) _location (`KismetMathLibrary.MakeRotator` 0.0 0.0 _returnvalue_yaw) false null))
        (bind _output_get (set `self.SpawnedAI` _returnvalue_3))
        (set `self.bDefeated` false)
        (bind _asbp_enemy_base (cast `/Game/Blueprints/Enemy/BP_Enemy_Base` _output_get))
        (add `/Game/Blueprints/Enemy/BP_Enemy_Base.OnDeath` _asbp_enemy_base (delegate `SetDefeated`))))))

(event `SetDefeated`
  (set `self.bDefeated` true)
  (`KismetSystemLibrary.PrintString` "Enemy has been Defeated"))

(fn `UserConstructionScript`
  (bind _extentz (`self.ExtentZ`))
  (`BoxComponent.SetBoxExtent` (`self.Box`) (`KismetMathLibrary.MakeVector` (`self.ExtentX`) (`self.ExtentY`) _extentz) true)
  (`SceneComponent.K2_SetRelativeLocation` (`self.Box`) (`KismetMathLibrary.MakeVector` 0.0 0.0 _extentz) false false))