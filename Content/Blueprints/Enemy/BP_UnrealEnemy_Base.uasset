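; Base enemy character that handles health, hit reactions, weapon wielding and death, leaving Attack empty for child classes.
; BPC damage system component drives HitResponse and Death, which set AI controller states for frozen, attacking and dead.
; BeginPlay creates the health bar widget, socket-attached weapon and patrol route; damage shows the bar on a hide timer.
; Death ragdolls the mesh, detaches the weapon and fades dynamic materials via timeline before destroying the actor.
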(event `self.ReceiveBeginPlay`
  ;[0 0.1277 0.1719] Create Health Bar Widget
  (bind _returnvalue (`|CreateWidget` "/Game/UI/W_HealthBar.W_HealthBar_C" null self))
  (`WidgetComponent.SetWidget` (`self.HealthBar`) _returnvalue)
  (bind _asaic_unreal_enemy_base (cast `/Game/Blueprints/Enemy/AI/AIC_UnrealEnemy_Base` (`AIBlueprintHelperLibrary.GetAIController` self)))
  (set `self.AICEnemyBase` _asaic_unreal_enemy_base)
  (`self.Wield Weapon`)
  (`self.CreatePatrolRoute`))

(event `HitResponse`
  (params (DamageCauser :type "Actor Object Reference"))
  ;[0.224 0.1225 0.1225] Impact Animation when Hit (Frozen)
  (`MovementComponent.StopMovementImmediately` (`self.CharacterMovement`))
  (if (not (`self.bIsAttacking`))
    (`/Game/Blueprints/Enemy/AI/AIC_UnrealEnemy_Base.SetStateAsFrozen` (`self.AICEnemyBase`))
    (`|PlayMontage` (`self.Mesh`) (`KismetArrayLibrary.Array_Random` (`self.ImpactAnimations`))
      (:`OnCompleted`
        (`/Game/Blueprints/Enemy/AI/AIC_UnrealEnemy_Base.SetStateAsAttacking` (`self.AICEnemyBase`) DamageCauser false)))))

(event `Attack`
  ;[0.1892 0.05327 0.4167] Attack Event to be used by children.
)

(event `Wield Weapon`
  ;[0.1875 0.1515 0] Wield Weapon if "Weapon" is valid
  (bind _weapon (`self.Weapon`)
    (:`then`
      (bind _returnvalue (`|SpawnActorFromClass` _weapon (`self.GetTransform`) "Undefined" "MultiplyWithRoot" null null))
      (bind _output_get (set `self.WeaponObject` _returnvalue))
      (`/Game/Blueprints/Weapons/BP_Weapon.SetupWeapon` _output_get self (`self.AttackDamageAmount`))
      (bind _returnvalue_2 (`self.K2_AttachToComponent` _output_get (`self.Mesh`) "hand_r_sword_socket" "SnapToTarget" "SnapToTarget" "SnapToTarget" true))
      (set `self.bIsWieldingWeapon` _returnvalue_2))
    (:`else`)))

(event `Death`
  (bind _mesh (`self.Mesh`))
  ;[0.09375 0 0] Death
  (`/Game/Blueprints/Enemy/AI/AIC_UnrealEnemy_Base.SetStateAsDead` (`self.AICEnemyBase`))
  (`self.OnDeath`)
  (`BrainComponent.StopLogic` (`AIController.BrainComponent` (`self.AICEnemyBase`)) "")
  (bind _weaponobject (`self.WeaponObject`)
    (:`then`
      (`/Game/Blueprints/Weapons/BP_Weapon.DetachWeapon` _weaponobject)
      ;;[0.224 0.5207 1] Detach Weapon
      (`/Game/Blueprints/Weapons/BP_Weapon.WeaponDecay` _weaponobject (`self.AfterDeathStartDecay`) (`self.DecayTime`)))
    (:`else`
      _))
  (`PrimitiveComponent.SetSimulatePhysics` _mesh true)
  ;;[0.375 0.2908 0] Ragdoll
  (`PrimitiveComponent.SetCollisionEnabled` _mesh "QueryAndPhysics")
  (`self.HealthBarInvisible`)
  ;;[0 0.09948 0.1562] Remove Widget and collision
  (`PrimitiveComponent.SetCollisionEnabled` (`self.CapsuleComponent`) "NoCollision")
  (`KismetSystemLibrary.Delay` (`self.AfterDeathStartDecay`))
  ;;[0.1875 0.1875 0.1875] Decay over time
  (`TimelineComponent.SetPlayRate` (`self.Fade`) (/ 1.0 (`self.DecayTime`)))
  (bind (_direction _fade) (`Timeline|Fade` :!via `PlayFromStart`)
    (:`Update`
      (`MaterialInstanceDynamic.SetScalarParameterValue` (`self.MeshMaterialOne`) "Fade" _fade)
      (`MaterialInstanceDynamic.SetScalarParameterValue` (`self.MeshMaterialTwo`) "Fade" _fade))
    (:`Finished`
      (`KismetSystemLibrary.Delay` 0.2)
      (`self.K2_DestroyActor`))))

(fn `CreatePatrolRoute`
  (`self.PatrolRoute`
    (:`then`)
    (:`else`
      (bind _returnvalue (`|SpawnActorFromClass` (`self.PatroulRouteClass`) (`SceneComponent.K2_GetComponentToWorld` (`self.Mesh`)) "Undefined" "MultiplyWithRoot" null null))
      (set `self.PatrolRoute` _returnvalue))))

(fn `GetCurrentHealth`
  (returns (Health :type Integer))
  (return (`/Game/Blueprints/DamageSystem/BPC_DamageSystem.Health` (`self.BPC_DamageSystem`))))

(fn `GetMaxHealth`
  (returns (MaxHealth :type Integer))
  (return (`/Game/Blueprints/DamageSystem/BPC_DamageSystem.MaxHealth` (`self.BPC_DamageSystem`))))

(fn `GetPatrolRoute`
  (returns (PatrolRoute :type "/Game/Blueprints/Enemy/AI/BP_PatrolRoute Object Reference"))
  (return (`self.PatrolRoute`)))

(fn `Heal`
  (params (Amount :type Integer))
  (returns (NewHealth :type Integer))
  (bind _newhealth (`/Game/Blueprints/DamageSystem/BPC_DamageSystem.Heal` (`self.BPC_DamageSystem`) Amount))
  (return _newhealth))

(fn `HealthBarInvisible`
  (`SceneComponent.SetVisibility` (`self.HealthBar`) false false)
  (`KismetSystemLibrary.K2_PauseTimerHandle` (`self.HealthBarTimerHandle`)))

(fn `IsDead`
  (returns (bDead :type Boolean))
  (return (`/Game/Blueprints/DamageSystem/BPC_DamageSystem.bIsDead` (`self.BPC_DamageSystem`))))

(fn `RemovePatrolRoute`
  (bind _patrolroute (`self.PatrolRoute`)
    (:`then`
      (`self.K2_DestroyActor` _patrolroute)
      (set `self.PatrolRoute` null))
    (:`else`)))

(fn `SetMovementSpeed`
  (params (Speed :type "/Game/Blueprints/Enemy/AI/Enums/E_MovementSpeed Enum" :default "NewEnumerator0"))
  (returns (SpeedValue :type "Float (double-precision)"))
  (bind _output_get (set `CharacterMovementComponent.MaxWalkSpeed` (select `/Game/Blueprints/Enemy/AI/Enums/E_MovementSpeed` Speed :`NewEnumerator1` 230.0 :`NewEnumerator2` 500.0 :!type "Float (single-precision)") (`self.CharacterMovement`)))
  (return _output_get))

(fn `TakeDamage`
  (params (Amount :type Integer) (Causer :type "Actor Object Reference") (Location :type "Vector Structure"))
  (returns (WasDamaged :type Boolean))
  (`SceneComponent.SetVisibility` (`self.HealthBar`) true false)
  (bind _bwasdamaged (`/Game/Blueprints/DamageSystem/BPC_DamageSystem.TakeDamage` (`self.BPC_DamageSystem`) (make `/Game/Blueprints/DamageSystem/S_DamageInfo` Amount) Causer))
  (if _bwasdamaged
    (`self.HitResponse` Causer)
    (`GameplayStatics.SpawnEmitterAtLocation` "/Game/StarterContent/Particles/P_Explosion.P_Explosion" Location (struct) (0.2 0.2 0.2))
    (bind _returnvalue (`KismetSystemLibrary.K2_SetTimer` null "HealthBarInvisible" (`self.HealthBarVisibilityTimer`)))
    (set `self.HealthBarTimerHandle` _returnvalue)
    (return _bwasdamaged)))

(fn `UserConstructionScript`
  (bind _bpc_damagesystem (`self.BPC_DamageSystem`))
  (bind _output_get (set `/Game/Blueprints/DamageSystem/BPC_DamageSystem.MaxHealth` (`self.MaxHealth`) _bpc_damagesystem))
  (set `/Game/Blueprints/DamageSystem/BPC_DamageSystem.Health` _output_get _bpc_damagesystem)
  (add `/Game/Blueprints/DamageSystem/BPC_DamageSystem.OnDeath` (`self.BPC_DamageSystem`) (`|CreateDelegate` :!event `Death`))
  (add `/Game/Blueprints/DamageSystem/BPC_DamageSystem.DamageResponse` (`self.BPC_DamageSystem`) (`|CreateDelegate` :!event `HitResponse`))
  (bind _returnvalue (`PrimitiveComponent.CreateDynamicMaterialInstance` (`self.Mesh`) 0 (`self.SourceMaterial_01`) "None"))
  (set `self.MeshMaterialOne` _returnvalue)
  (bind _returnvalue_2 (`PrimitiveComponent.CreateDynamicMaterialInstance` (`self.Mesh`) 1 (`self.SourceMaterial_02`) "None"))
  (set `self.MeshMaterialTwo` _returnvalue_2))