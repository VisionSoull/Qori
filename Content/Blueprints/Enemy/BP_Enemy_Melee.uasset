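; Weaponless melee enemy that attacks with an animation montage, flagged as wielding a weapon so it is able to attack.
; Montage notifies toggle the attack capsule's overlap events and clear the hit list; montage end notifies the Behavior Tree task.
; Overlaps accept damageable actors on the opposing side, once per window.
; A short forward sphere trace must confirm the target, supplying the impact point for damage and hit sound.
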(event `self.Attack`
  (`parent.Attack`)
  (bind _notifyname (`|PlayMontage` (`self.Mesh`) "/Game/Characters/Animations/Azeman/AM_Azeman_Attack.AM_Azeman_Attack")
    (:`then`
      (set `self.bIsAttacking` true))
    (:`OnCompleted`
      (set `self.bIsAttacking` false :!label _label)
      (`self.OnAttackEnd`) ; Subscriber on Behavior Tree Task
    )
    (:`OnInterrupted`
      (goto _label))
    (:`OnNotifyBegin`
      (switch `name` _notifyname
        (:`Slash`
          (`self.OverlapEvent` true))))
    (:`OnNotifyEnd`
      (switch `name` _notifyname
        (:`Slash`
          (`self.OverlapEvent` false)
          (`KismetArrayLibrary.Array_Clear` (`self.HitTargets`)))))))

(event `self.AttackCapsule.OnComponentBeginOverlap`
  (params (OverlappedComponent :type "PrimitiveComponent Object Reference") (OtherActor :type "Actor Object Reference") (OtherComp :type "PrimitiveComponent Object Reference") (OtherBodyIndex :type Integer) (bFromSweep :type Boolean) (SweepResult :type "HitResult Structure (by ref)"))
  (bind (_asbpi_damageable _bsuccess) (cast `/Game/Blueprints/DamageSystem/BPI_Damageable` OtherActor :!pure true))
  (if (and (and _bsuccess (!= OtherActor self)) (!= (`KismetMathLibrary.ClassIsChildOf` (`GameplayStatics.GetObjectClass` self) "/Game/Blueprints/Enemy/BP_Enemy_Base.BP_Enemy_Base_C") (`KismetMathLibrary.ClassIsChildOf` (`GameplayStatics.GetObjectClass` OtherActor) "/Game/Blueprints/Enemy/BP_Enemy_Base.BP_Enemy_Base_C")))
    (if (not (`KismetArrayLibrary.Array_Contains` (`self.HitTargets`) _asbpi_damageable))
      (`KismetArrayLibrary.Array_AddUnique` (`self.HitTargets`) _asbpi_damageable)
      (bind _outhits (`KismetSystemLibrary.SphereTraceMultiForObjects` (`SceneComponent.K2_GetComponentLocation` (`self.CapsuleComponent`)) (+ (`SceneComponent.K2_GetComponentLocation` (`self.CapsuleComponent`)) (* (`SceneComponent.GetForwardVector` (`self.CapsuleComponent`)) 100.0)) 10.0 (`|MakeArray` "ObjectTypeQuery3" :!type "EObjectTypeQuery Enum") false (`|MakeArray` self :!type "Actor Object Reference") "ForDuration" true (struct :`R` 1.0 :`A` 1.0) (struct :`G` 1.0 :`A` 1.0) 1.0))
      (for _array_element _outhits
        (bind (_bblockinghit _binitialoverlap _time _distance _location _impactpoint _normal _impactnormal _physmat _hitactor) (`GameplayStatics.BreakHitResult` _array_element))
        (if (== _asbpi_damageable _hitactor)
          (`|ExecutionSequence`
            (:`then_0`
              (`/Game/Blueprints/DamageSystem/BPI_Damageable.TakeDamage` _asbpi_damageable (`self.AttackDamageAmount`) self _impactpoint)
              (`GameplayStatics.PlaySoundAtLocation` (`self.HitSound`) _impactpoint (struct) 1.0 1.0 0.0 null null null null))
            (:`then_1`
              (break))))))))

(fn `UserConstructionScript`
  (`parent.UserConstructionScript`)
  ;[1 1 1] This Enemy does not use a weapon. In order for this enemy to attack, this setup is necessary because it needs to wield a weapon to attack.
  (set `self.Weapon` null)
  (set `self.bIsWieldingWeapon` true))