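; Enemy actor that periodically attacks pawns in front of it with a sphere trace, sending damage and spawning an explosion, on a looping test timer.
; Health, healing and damage calls forward to BPCDamageSystem, and a health bar widget is created with the enemy as its damageable actor.
; On death it ragdolls, drops its widget and capsule collision, then fades both dynamic mesh materials via a timeline before destroying itself.
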(event `self.ReceiveBeginPlay`
  (`KismetSystemLibrary.K2_SetTimerDelegate` (delegate `Attack`) 2.0 true)
  ;[0 0.1277 0.1719] Create Health Bar Widget
  (bind _returnvalue (`|CreateWidget` "/Game/Blueprints/W_HealthBar.W_HealthBar_C" null self))
  (`WidgetComponent.SetWidget` (`self.Widget`) _returnvalue))

(event `Attack`
  (bind _returnvalue (`self.K2_GetActorLocation`))
  ;[0.06771 0 0.04434] Attack By Time (For testing purposes)
  (if (not (`/Game/Blueprints/DamageSystem/BPC_DamageSystem.bIsDead` (`self.BPC_DamageSystem`)))
    (bind (_outhit _returnvalue_2) (`KismetSystemLibrary.SphereTraceSingleForObjects` :`Start` _returnvalue :`End` (+ _returnvalue (* (`self.GetActorForwardVector`) 200.0)) :`Radius` 20.0 :`ObjectTypes` (`|MakeArray` "ObjectTypeQuery3" :!type "EObjectTypeQuery Enum") :`DrawDebugType` "ForDuration" :`TraceColor` (struct :`R` 1.0 :`B` 0.979897 :`A` 1.0) :`TraceHitColor` (struct :`G` 0.846483 :`B` 1.0 :`A` 1.0) :`DrawTime` 0.2))
    (if _returnvalue_2
      (bind (_bblockinghit _binitialoverlap _time _distance _location _impactpoint _normal _impactnormal _physmat _hitactor) (`GameplayStatics.BreakHitResult` _outhit))
      (message `/Game/Blueprints/DamageSystem/BPI_Damageable.TakeDamage` _hitactor (make `/Game/Blueprints/DamageSystem/S_DamageInfo` (`self.AttackDamage`)))
      (`GameplayStatics.SpawnEmitterAtLocation` "/Game/StarterContent/Particles/P_Explosion.P_Explosion" _location))))

(event `Death`
  (bind _mesh (`self.Mesh`))
  ;[0.09375 0 0] Death
  ;;[0.375 0.2908 0] Ragdoll
  (`PrimitiveComponent.SetSimulatePhysics` _mesh true)
  (`PrimitiveComponent.SetCollisionEnabled` _mesh "QueryAndPhysics")
  ;;[0 0.09948 0.1562] Remove Widget and collision
  (`ActorComponent.K2_DestroyComponent` (`self.Widget`))
  (`PrimitiveComponent.SetCollisionEnabled` (`self.CapsuleComponent`) "NoCollision")
  ;;[0.1875 0.1875 0.1875] Decay over time
  (`KismetSystemLibrary.Delay` (`self.AfterDeathStartDecay`))
  (`TimelineComponent.SetPlayRate` (`self.Fade`) (/ 1.0 (`self.DecayTime`)))
  (bind (_direction _fade) (`Timeline|Fade` :!via `PlayFromStart`)
    (:`Update`
      (`MaterialInstanceDynamic.SetScalarParameterValue` (`self.MeshMaterialOne`) "Fade" _fade)
      (`MaterialInstanceDynamic.SetScalarParameterValue` (`self.MeshMaterialTwo`) "Fade" _fade))
    (:`Finished`
      (`KismetSystemLibrary.Delay` 0.5)
      (`self.K2_DestroyActor`))))

(fn `GetCurrentHealth`
  (returns (Health :type Integer))
  (return (`/Game/Blueprints/DamageSystem/BPC_DamageSystem.Health` (`self.BPC_DamageSystem`))))

(fn `GetMaxHealth`
  (returns (MaxHealth :type Integer))
  (return (`/Game/Blueprints/DamageSystem/BPC_DamageSystem.MaxHealth` (`self.BPC_DamageSystem`))))

(fn `Heal`
  (params (Amount :type Integer))
  (returns (NewHealth :type Integer))
  (bind _newhealth (`/Game/Blueprints/DamageSystem/BPC_DamageSystem.Heal` (`self.BPC_DamageSystem`) Amount))
  (return _newhealth))

(fn `TakeDamage`
  (params (DamageInfo :type "/Game/Blueprints/DamageSystem/S_DamageInfo Structure"))
  (returns (WasDamaged :type Boolean))
  (bind _bwasdamaged (`/Game/Blueprints/DamageSystem/BPC_DamageSystem.TakeDamage` (`self.BPC_DamageSystem`) DamageInfo))
  (return _bwasdamaged))

(fn `UserConstructionScript`
  (add `/Game/Blueprints/DamageSystem/BPC_DamageSystem.OnDeath` (`self.BPC_DamageSystem`) (`|CreateDelegate` :!event `Death`))
  (bind _returnvalue (`PrimitiveComponent.CreateDynamicMaterialInstance` (`self.Mesh`) 0 "/Game/Characters/Mannequins/Materials/Instances/Manny/MI_Manny_01.MI_Manny_01" "None"))
  (set `self.MeshMaterialOne` _returnvalue)
  (bind _returnvalue_2 (`PrimitiveComponent.CreateDynamicMaterialInstance` (`self.Mesh`) 1 "/Game/Characters/Mannequins/Materials/Instances/Manny/MI_Manny_02.MI_Manny_02" "None"))
  (set `self.MeshMaterialTwo` _returnvalue_2))