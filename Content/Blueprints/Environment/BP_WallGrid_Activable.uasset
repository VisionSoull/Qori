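; BP_WallGrid_Activable is a modular wall row with one door slot that Activate toggles between jail-cell and doorway meshes.
; The construction script spawns wall segments along X from random meshes, placing the door at DoorInIndex and spacing each by its own bounds.
; A randomly rotated corner pillar caps the start when the first segment is a wall.
; The end-pillar logic is disconnected and marked as broken.
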(event `/Game/Blueprints/Interfaces/BPI_Activable.Activate`
  (if (`self.bDoorClosed`)
    (`StaticMeshComponent.SetStaticMesh` (`self.Door`) "/Game/Meshes/DoorWay.DoorWay")
    (set `self.bDoorClosed` false)
    (else
      (`StaticMeshComponent.SetStaticMesh` (`self.Door`) "/Game/Meshes/JailCell.JailCell")
      (set `self.bDoorClosed` true))))

(fn `UserConstructionScript`
  (for _index (range 1 (+ (`self.NumberOfWalls`) 1))
    (bind _returnvalue (`AddComponent|NODE_AddStaticMeshComponent-0`))
    (if (== _index (`self.DoorInIndex`))
      (if (`self.bDoorClosed`)
        (`StaticMeshComponent.SetStaticMesh` _returnvalue "/Game/Meshes/JailCell.JailCell")
        (else
          (`StaticMeshComponent.SetStaticMesh` _returnvalue "/Game/Meshes/DoorWay.DoorWay")))
      (set `self.Door` _returnvalue)
      (bind (_min _max) (`StaticMeshComponent.GetLocalBounds` _returnvalue))
      (bind _returnvalue_x (`KismetMathLibrary.BreakVector` (- _max _min)))
      (`SceneComponent.K2_SetRelativeLocation` _returnvalue (`KismetMathLibrary.MakeVector` (* (`self.Coord`) _returnvalue_x)) false false :!label _label)
      (`/Engine/EditorBlueprintResources/StandardMacros.IncrementInt` (`self.Coord`))
      (else
        (`StaticMeshComponent.SetStaticMesh` _returnvalue (`KismetArrayLibrary.Array_Random` (`self.WallMesh`)))
        (`|ExecutionSequence`
          (:`then_0`
            (goto _label))
          (:`then_1`
            (if (== _index 1)
              (bind _returnvalue_2 (`AddComponent|NODE_AddStaticMeshComponent-3`))
              (`StaticMeshComponent.SetStaticMesh` _returnvalue_2 "/Game/Meshes/CornerPillar.CornerPillar")
              (`SceneComponent.K2_SetRelativeLocationAndRotation` _returnvalue_2 (`KismetMathLibrary.MakeVector` (.x _min)) (`KismetMathLibrary.MakeRotator` 0.0 0.0 (`KismetArrayLibrary.Array_Random` (`self.RandomRotation`))) false false))))))))