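; BP_Torch_Activable is an environment torch whose light and effect can be toggled.
; The construction script applies the LightColor, Radius and Intensity variables to its PointLight.
; The Activate event calls VisibleNotVisible, which flips the visibility of the PointLight and FXSTorches, propagating to children only for the latter.
; Because it toggles rather than sets visibility, each activation reverses the current state.
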(event `/Game/Blueprints/Interfaces/BPI_Activable.Activate`
  (`self.Visible/NotVisible`))

(fn `UserConstructionScript`
  (`LightComponent.SetLightColor` (`self.PointLight`) (`self.LightColor`) true)
  (`LocalLightComponent.SetAttenuationRadius` (`self.PointLight`) (`self.Radius`))
  (`LightComponent.SetIntensity` (`self.PointLight`) (`self.Intensity`)))

(fn `Visible/NotVisible`
  (`SceneComponent.ToggleVisibility` (`self.PointLight`) false)
  (`SceneComponent.ToggleVisibility` (`self.FXS_Torches`) true))