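; BP_Torch is an environment torch actor with a point light and a torch FX component.
; The construction script applies exposed color, radius and intensity values to the light, and uses IsLitUp to show or hide both the light and the FX, including FX children.
; A separate VisibleNotVisible function toggles only the light's visibility, leaving the FX untouched.
; The event graph holds no active logic.
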(fn `UserConstructionScript`
  (`LightComponent.SetLightColor` (`self.PointLight`) (`self.LightColor`) true)
  (`LocalLightComponent.SetAttenuationRadius` (`self.PointLight`) (`self.Radius`))
  (`LightComponent.SetIntensity` (`self.PointLight`) (`self.Intensity`))
  (`SceneComponent.SetVisibility` (`self.PointLight`) (`self.bIsLitUp`) false)
  (`SceneComponent.SetVisibility` (`self.FXS_Torches`) (`self.bIsLitUp`) true))

(fn `Visible/NotVisible`
  (`SceneComponent.ToggleVisibility` (`self.PointLight`) false))