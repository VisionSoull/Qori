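; Environment actor that builds a GridSizeX by GridSizeY floor of static mesh tiles in its construction script.
; Each cell gets a new component with a random mesh from FloorMesh and a random yaw from RandomRotationValues.
; Tiles fill row by row, spaced by the chosen mesh's local bounds, so even tiling relies on same-sized meshes.
; The random picks are unseeded, and the event graph has no logic.
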(event `self.ReceiveBeginPlay`)

(fn `UserConstructionScript`
  (for _ (range 1 (+ (* (`self.GridSizeX`) (`self.GridSizeY`)) 1))
    (if (> (`self.XCoord`) (- (`self.GridSizeX`) 1)) :!label _label
      (set `self.XCoord` 0)
      (`/Engine/EditorBlueprintResources/StandardMacros.IncrementInt` (`self.YCoord`)
        (:`  `
          (goto _label)))
      (else
        (bind _returnvalue (`AddComponent|NODE_AddStaticMeshComponent-0`))
        (`StaticMeshComponent.SetStaticMesh` _returnvalue (`KismetArrayLibrary.Array_Random` (`self.FloorMesh`)))
        (bind (_min _max) (`StaticMeshComponent.GetLocalBounds` _returnvalue))
        (bind (_returnvalue_x _returnvalue_y) (`KismetMathLibrary.BreakVector` (- _max _min)))
        (`SceneComponent.K2_SetRelativeLocationAndRotation` _returnvalue (`KismetMathLibrary.MakeVector` (* (`self.XCoord`) _returnvalue_x) (* (`self.YCoord`) _returnvalue_y)) (`KismetMathLibrary.MakeRotator` 0.0 0.0 (`KismetArrayLibrary.Array_Random` (`self.RandomRotationValues`))) false false)
        (`/Engine/EditorBlueprintResources/StandardMacros.IncrementInt` (`self.XCoord`))))))