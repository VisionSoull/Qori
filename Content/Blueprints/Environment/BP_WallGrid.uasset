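; BP_WallGrid is an environment Blueprint that procedurally builds a straight row of wall meshes along local X.
; Its construction script adds NumberOfWalls static mesh components with randomly picked meshes, each offset by a running counter times its own bounds width.
; A corner pillar with random yaw starts the row, and an optional end pillar applies only to single-wall rows.
; The random picks are unseeded, so layouts can change on reconstruction.
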(fn `UserConstructionScript`
  (for _index (range 1 (+ (`self.NumberOfWalls`) 1))
    (bind _returnvalue (`AddComponent|NODE_AddStaticMeshComponent-0`))
    (`|ExecutionSequence`
      (:`then_0`
        (`StaticMeshComponent.SetStaticMesh` _returnvalue (`KismetArrayLibrary.Array_Random` (`self.WallMesh`)))
        (bind (_min _max) (`StaticMeshComponent.GetLocalBounds` _returnvalue))
        (bind _returnvalue_x (`KismetMathLibrary.BreakVector` (- _max _min)))
        (`SceneComponent.K2_SetRelativeLocation` _returnvalue (`KismetMathLibrary.MakeVector` (* (`self.Coord`) _returnvalue_x)) false false)
        (`/Engine/EditorBlueprintResources/StandardMacros.IncrementInt` (`self.Coord`)))
      (:`then_1`
        (if (== _index 1)
          (bind _returnvalue_2 (`AddComponent|NODE_AddStaticMeshComponent-3`))
          (`StaticMeshComponent.SetStaticMesh` _returnvalue_2 "/Game/Meshes/CornerPillar.CornerPillar")
          (`SceneComponent.K2_SetRelativeLocationAndRotation` _returnvalue_2 (`KismetMathLibrary.MakeVector` (.x _min)) (`KismetMathLibrary.MakeRotator` 0.0 0.0 (`KismetArrayLibrary.Array_Random` (`self.RandomRotation`))) false false)))
      (:`then_2`
        ;[1 1 1] Corner Pillar if there is only 1 wall
        (if (and (<= (`self.NumberOfWalls`) 1) (`self.bHasEndPillar (1 Wall)`))
          (bind _returnvalue_3 (`AddComponent|NODE_AddStaticMeshComponent-5`))
          (`StaticMeshComponent.SetStaticMesh` _returnvalue_3 "/Game/Meshes/CornerPillar.CornerPillar")
          (`SceneComponent.K2_SetRelativeLocationAndRotation` _returnvalue_3 (`KismetMathLibrary.MakeVector` (* (`self.Coord`) (.x _max))) (`KismetMathLibrary.MakeRotator` 0.0 0.0 (`KismetArrayLibrary.Array_Random` (`self.RandomRotation`))) false false))))))