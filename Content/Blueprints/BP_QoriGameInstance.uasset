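; Game instance for Qori that owns the save game, handling loading, saving, progress deletion and reopening the saved level.
; Init loads or creates the BP_SaveGame slot, seeding default audio volumes, and loads user settings.
; Saving snapshots player location, level, data table row, and statue, plate manager and persistent spawner states, writing sync or async.
; Audio volumes persist in the same save, survive deletion, and apply through sound mix overrides.
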(event `self.ReceiveInit`
  (`self.LoadGameData` false)
  (bind _returnvalue (`GameUserSettings.GetGameUserSettings`))
  (`GameUserSettings.LoadSettings` _returnvalue false))

(event `/Game/Blueprints/SaveGame/BPI_SaveGame.LoadGameData`
  (params (bASync :type Boolean))
  ;[0.9034 1 0.0904] Load Game
  (bind _bexists (`self.DoesSaveGameExist`))
  (if _bexists
    (if bASync
      (bind _savegame (`AsyncActionHandleSaveGame.AsyncLoadGameFromSlot` (`self.Slot Name`))
        (:`Completed`
          (bind _asbp_save_game (cast `/Game/Blueprints/SaveGame/BP_SaveGame` _savegame))
          (set `self.SaveGameReference` _asbp_save_game)
          (`self.GetAudioSettingsFromSaveGame`)
          (`self.OnGameLoaded`)))
      (else
        (bind _returnvalue (`GameplayStatics.LoadGameFromSlot` (`self.Slot Name`)))
        (bind _asbp_save_game_2 (cast `/Game/Blueprints/SaveGame/BP_SaveGame` _returnvalue))
        (set `self.SaveGameReference` _asbp_save_game_2)
        (`self.GetAudioSettingsFromSaveGame`)))
    (else
      (bind _returnvalue_2 (`GameplayStatics.CreateSaveGameObject` "/Game/Blueprints/SaveGame/BP_SaveGame.BP_SaveGame_C"))
      (set `self.SaveGameReference` _returnvalue_2)
      (`/Game/Blueprints/SaveGame/BPI_SaveGame.SaveAudioSettings` 1.0 1.0 1.0) ; Default Audio Volumes for the First Time Opening the Game
    )))

(event `/Game/Blueprints/SaveGame/BPI_SaveGame.SaveGameData`
  (params (bAsync :type Boolean))
  ;[0.1882 0.5469 1] Save into Save Game Reference
  (`self.Save Data`)
  (`/Engine/EditorBlueprintResources/StandardMacros.IsValid` (`self.SaveGameReference`)
    (:`Is Valid`
      _)
    (:`Is Not Valid`
      (`GameplayStatics.CreateSaveGameObject` "/Game/Blueprints/SaveGame/BP_SaveGame.BP_SaveGame_C")))
  (`/Game/Blueprints/SaveGame/BP_SaveGame.SaveGame` (`self.SaveGameReference`) (`self.PlayerLocation_GI`) (`self.StatueRotations_GI`) (`self.PlatesManagerStates_GI`) (`self.PersistentSpawnerStates_GI`) (`self.Savedlevel_GI`) (`self.DataTableRowName_GI`))
  (if bAsync
    (`AsyncActionHandleSaveGame.AsyncSaveGameToSlot` (`self.SaveGameReference`) (`self.Slot Name`)
      (:`Completed`
        _))
    (else
      (`GameplayStatics.SaveGameToSlot` (`self.SaveGameReference`) (`self.Slot Name`))))
  (`self.OnGameSaved` (`self.SaveGameReference`)))

(event `Save Data`
  ;[0 0.3333 0.03108] Save Game
  (set `self.PlayerLocation_GI` (`Actor.K2_GetActorLocation` (`GameplayStatics.GetPlayerPawn` 0)))
  (bind _returnvalue (`GameplayStatics.GetCurrentLevelName` true))
  (set `self.Savedlevel_GI` (`KismetStringLibrary.Conv_StringToName` _returnvalue))
  (bind _rowname (message `/Game/Blueprints/Interfaces/BPI_TasksHandler.GetRowName` (`GameplayStatics.GetGameMode`)))
  (set `self.DataTableRowName_GI` _rowname)
  (`KismetArrayLibrary.Array_Clear` (`self.StatueRotations_GI`))
  (bind _outactors (`GameplayStatics.GetAllActorsOfClass` "/Game/Blueprints/Puzzles/Statues/BP_Statue.BP_Statue_C"))
  (for _array_element _outactors
    (`KismetArrayLibrary.Array_AddUnique` (`self.StatueRotations_GI`) (make `/Game/Blueprints/SaveGame/Structures/S_StatueRotations` (`|ConvertAsset` _array_element) (`/Game/Blueprints/Puzzles/Statues/BP_Statue.CurrentRotation` _array_element))))
  (`KismetArrayLibrary.Array_Clear` (`self.PlatesManagerStates_GI`))
  (bind _outactors_2 (`GameplayStatics.GetAllActorsOfClass` "/Game/Blueprints/Puzzles/Plates/BP_PlatesManager.BP_PlatesManager_C"))
  (for _array_element_2 _outactors_2
    (`KismetArrayLibrary.Array_AddUnique` (`self.PlatesManagerStates_GI`) (make `/Game/Blueprints/SaveGame/Structures/S_PlateManagerStates` (`|ConvertAsset` _array_element_2) (`/Game/Blueprints/Puzzles/Plates/BP_PlatesManager.bIsComplete` _array_element_2))))
  (`KismetArrayLibrary.Array_Clear` (`self.PersistentSpawnerStates_GI`))
  (bind _outactors_3 (`GameplayStatics.GetAllActorsOfClass` "/Game/Blueprints/Enemy/Spawners/Parents/BP_PersistentSpawner.BP_PersistentSpawner_C"))
  (for _array_element_3 _outactors_3
    (`KismetArrayLibrary.Array_AddUnique` (`self.PersistentSpawnerStates_GI`) (make `/Game/Blueprints/SaveGame/Structures/S_PersistentSpawnerStates` _array_element_3 (`/Game/Blueprints/Enemy/Spawners/Parents/BP_PersistentSpawner.bDefeated` _array_element_3)))))

(event `/Game/Blueprints/SaveGame/BPI_SaveGame.DeleteSaveGame`
  (bind _savegamereference (`self.SaveGameReference`))
  ;[0.25 0 0] Delete Save Game Info while Keeping Settings
  (`/Game/Blueprints/SaveGame/BP_SaveGame.Delete Save Game` _savegamereference)
  (`GameplayStatics.SaveGameToSlot` _savegamereference (`self.Slot Name`)))

(event `/Game/Blueprints/SaveGame/BPI_SaveGame.LoadLevel`
  ;[0.1874 1 0.9901] Load Level
  (`GameplayStatics.OpenLevel` (`/Game/Blueprints/SaveGame/BP_SaveGame.SavedLevel` (`self.SaveGameReference`))))

(event `/Game/Blueprints/SaveGame/BPI_SaveGame.SaveAudioSettings`
  (params (Master :type "Float (double-precision)") (Music :type "Float (double-precision)") (Effects :type "Float (double-precision)"))
  (`/Game/Blueprints/SaveGame/BP_SaveGame.SaveAudioSettings` (`self.SaveGameReference`) Master Music Effects)
  (`GameplayStatics.SaveGameToSlot` (`self.SaveGameReference`) (`self.Slot Name`)))

(fn `DoesSaveGameExist`
  (returns (bExists :type Boolean))
  (bind _returnvalue (`GameplayStatics.DoesSaveGameExist` (`self.Slot Name`)))
  (return _returnvalue))

(fn `GetAudioSettingsFromSaveGame`
  (bind (_volumemaster _volumemusic _volumeeffects) (`/Game/Blueprints/SaveGame/BP_SaveGame.GetAudioSettings` (`self.SaveGameReference`)))
  (set `self.VolumeMaster_GI` _volumemaster)
  (set `self.VolumeMusic_GI` _volumemusic)
  (set `self.VolumeEffects_GI` _volumeeffects))

(fn `GetGameData`
  (returns (SaveGameData :type "/Game/Blueprints/SaveGame/BP_SaveGame Object Reference"))
  (return (`self.SaveGameReference`)))

(fn `SetAudioVolumes`
  (`GameplayStatics.SetSoundMixClassOverride` "/Game/Sound/SoundMix.SoundMix" "/Game/Sound/Classes/Master.Master" (`self.VolumeMaster_GI`))
  (`GameplayStatics.SetSoundMixClassOverride` "/Game/Sound/SoundMix.SoundMix" "/Game/Sound/Classes/Music.Music" (`self.VolumeMusic_GI`))
  (`GameplayStatics.SetSoundMixClassOverride` "/Game/Sound/SoundMix.SoundMix" "/Game/Sound/Classes/SFX.SFX" (`self.VolumeEffects_GI`)))