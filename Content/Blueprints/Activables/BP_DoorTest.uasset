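; BP_DoorTest is an activable test door that rotates its mesh around yaw when activated.
; Activate captures the current world rotation of SMDoor and adds AmountToRotate to its yaw to form the target.
; The TimeToRotate timeline then plays from start, lerping the mesh between the two rotations.
; There is no closing logic, so each activation takes the current rotation as its new starting point.
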(event `/Game/Blueprints/Interfaces/BPI_Activable.Activate`
  (bind _output_get (set `self.InitialRotation` (`SceneComponent.K2_GetComponentRotation` (`self.SM_Door`))))
  (set `self.FinalRotation` (`KismetMathLibrary.MakeRotator` (.roll _output_get) (.pitch _output_get) (+ (.yaw _output_get) (`self.AmountToRotate`))))
  (bind (_direction _time) (`Timeline|TimeToRotate` :!via `PlayFromStart`)
    (:`Update`
      (`SceneComponent.K2_SetWorldRotation` (`self.SM_Door`) (`KismetMathLibrary.RLerp` (`self.InitialRotation`) (`self.FinalRotation`) _time) false false))))

(fn `UserConstructionScript`)