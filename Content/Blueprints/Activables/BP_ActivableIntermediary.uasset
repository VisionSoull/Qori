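; BP_ActivableIntermediary is a gate between connectors and activable actors, firing its targets once enough connectors have activated.
; BeginPlay counts unique connectors from ConnectorsList, and AddConnectortoList can register more and update that count.
; Each Activate call increments a counter; on matching the total, it sends ActivateMessage to every Activable and tells the GameMode to update the task list.
; The construction script clears Activables entries lacking BPI_Activable.
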(event `self.ReceiveBeginPlay`
  (set `self.ConnectorsActivated` 0)
  (for _array_element (`self.ConnectorsList`)
    (if (not (`KismetArrayLibrary.Array_Contains` (`self.UniqueConnectorsList`) _array_element))
      (`KismetArrayLibrary.Array_AddUnique` (`self.UniqueConnectorsList`) _array_element)))
  (set `self.NumberOfConnectors` (`KismetArrayLibrary.Array_Length` (`self.UniqueConnectorsList`))))

(event `/Game/Blueprints/Interfaces/BPI_Activable.Activate`
  (`/Engine/EditorBlueprintResources/StandardMacros.IncrementInt` (`self.ConnectorsActivated`)
    (:`  `
      (if (== (`self.ConnectorsActivated`) (`self.NumberOfConnectors`))
        (for _array_element (`self.Activables`)
          (message `/Game/Blueprints/Interfaces/BPI_Activable.Activate` _array_element))
        (message `/Game/Blueprints/Interfaces/BPI_TasksHandler.UpdateTaskList` (`GameplayStatics.GetGameMode`) self)))))

(event `/Game/Blueprints/Interfaces/BPI_ActivableIntermediary.AddConnectorToList`
  (params (Connector :type "Actor Object Reference"))
  (bind _returnvalue (`KismetArrayLibrary.Array_AddUnique` (`self.ConnectorsList`) Connector))
  (set `self.NumberOfConnectors` (+ _returnvalue 1)))

(fn `UserConstructionScript`
  (for (_array_element _array_index) (`self.Activables`)
    (`/Engine/EditorBlueprintResources/StandardMacros.IsValid` _array_element
      (:`Is Valid`
        (cast `/Game/Blueprints/Interfaces/BPI_Activable` _array_element
          (:`CastFailed`
            (`KismetArrayLibrary.Array_Set` (`self.Activables`) _array_index)))))))