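; Activable interact checkpoint that reveals a bonfire effect when activated.
; It hides the bonfire effect and its child components on BeginPlay, then shows them on Activate through a shared SetVisibility function.
; The construction script applies configurable color, radius and intensity to a point light, and a debug function toggles the effect's visibility.
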(event `self.ReceiveBeginPlay`
  (`self.SetVisibility` false))

(event `/Game/Blueprints/Interfaces/BPI_Activable.Activate`
  (`self.SetVisibility` true))

(fn `SetVisibility`
  (params (bNewVisibility :type Boolean))
  (`SceneComponent.SetVisibility` (`self.FXS_Bonfire`) bNewVisibility true))

(fn `ToggleEffectsVisibility(Debug)`
  (`SceneComponent.ToggleVisibility` (`self.FXS_Bonfire`) true))

(fn `UserConstructionScript`
  (`LightComponent.SetLightColor` (`self.PointLight`) (`self.LightColor`) true)
  (`LocalLightComponent.SetAttenuationRadius` (`self.PointLight`) (`self.Radius`))
  (`LightComponent.SetIntensity` (`self.PointLight`) (`self.Intensity`)))