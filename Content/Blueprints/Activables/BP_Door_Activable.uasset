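; BP_Door_Activable is an activable door that opens by moving its Cube vertically when Activate fires while it is not Active.
; A timeline, with play rate scaled by TimeToOpenInSeconds, lerps the Cube's relative location toward a new Z height.
; The timeline's Update path also shows a "Main Door opened" message through BP_QoriGameMode and clears it after a five-second delay.
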(event `/Game/Blueprints/Interfaces/BPI_Activable.Activate`
  (bind (_relativelocation_x _relativelocation_y) (`KismetMathLibrary.BreakVector` (`SceneComponent.RelativeLocation` (`self.Cube`))))
  (if (not (`self.bActive`))
    (set `self.InitialLocaiton` (`SceneComponent.RelativeLocation` (`self.Cube`)))
    (set `self.FinalLocation` (`KismetMathLibrary.MakeVector` _relativelocation_x _relativelocation_y (`self.NewVerticalRelativeLocation`)))
    (`TimelineComponent.SetPlayRate` (`self.TimeToOpen`) (/ 1.0 (`self.TimeToOpen(InSeconds)`)))
    (bind (_direction _time) (`Timeline|TimeToOpen` :!via `PlayFromStart`)
      (:`Update`
        (`SceneComponent.K2_SetRelativeLocation` (`self.Cube`) (`KismetMathLibrary.VLerp` (`self.InitialLocaiton`) (`self.FinalLocation`) _time) false false)
        (bind _asbp_qori_game_mode (cast `/Game/Blueprints/BP_QoriGameMode` (`GameplayStatics.GetGameMode`)))
        (`/Game/Blueprints/BP_QoriGameMode.SetInfoText` _asbp_qori_game_mode "The Main Door has been opened!")
        (`KismetSystemLibrary.Delay` 5.0)
        (`/Game/Blueprints/BP_QoriGameMode.SetInfoText` _asbp_qori_game_mode "")))))

(fn `UserConstructionScript`)