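; Manager for an ordered plate puzzle that activates a linked Activable actor when the last plate completes.
; Gathers plates overlapping PuzzleArea while OrderChangeable is set, numbers them and registers itself on each.
; SetNextPlateActive advances along the array, and completion makes every plate non-interactable.
; Construction validates the target's BPI_Activable interface; ResetPlates' loop has no array connected.
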(fn `AddPlate`
  (params (Plate :type "/Game/Blueprints/Plates/OlderLogics/BP_Plate_AreaMethod Object Reference"))
  (if (`self.bOrderChangeable`)
    (if (not (`KismetArrayLibrary.Array_Contains` (`self.AllPlates`) Plate))
      (`KismetArrayLibrary.Array_AddUnique` (`self.AllPlates`) Plate))
    (`self.Set Plate Numbers`)))

(fn `CompletePuzzle`
  (message `/Game/Blueprints/Interfaces/BPI_Activable.Activate` (`self.Activable`))
  (for _array_element (`self.AllPlates`)
    (`/Game/Blueprints/Plates/OlderLogics/BP_Plate_AreaMethod.SetNotInteractable` _array_element)))

(fn `RemovePlate`
  (params (Plate :type "/Game/Blueprints/Plates/OlderLogics/BP_Plate_AreaMethod Object Reference"))
  (`KismetArrayLibrary.Array_RemoveItem` (`self.AllPlates`) Plate)
  (`self.SetPuzzlePlates`))

(fn `ResetPlates`
  (for (_array_element _array_index) _
    (if (not (== _array_index 0))
      (`/Game/Blueprints/Plates/BP_Plate.Deactivate` _array_element))))

(fn `Set Plate Numbers`
  (for (_array_element _array_index) (`self.AllPlates`)
    (`/Game/Blueprints/Plates/OlderLogics/BP_Plate_AreaMethod.SetNumber` _array_element (+ _array_index 1))
    (`/Game/Blueprints/Plates/OlderLogics/BP_Plate_AreaMethod.SetPlatesManager` _array_element self)))

(fn `SetNextPlateActive`
  (params (CurrentPlate :type "/Game/Blueprints/Plates/OlderLogics/BP_Plate_AreaMethod Object Reference"))
  (bind _returnvalue (`KismetArrayLibrary.Array_Find` (`self.AllPlates`) CurrentPlate))
  ;[0.02604 0 0] Check if it is the last plate of the puzzle
  (if (== (`KismetArrayLibrary.Array_LastIndex` (`self.AllPlates`)) _returnvalue)
    (`self.CompletePuzzle`)
    (else
      (`/Game/Blueprints/Plates/OlderLogics/BP_Plate_AreaMethod.SetActive` (`|GetArrayItem` (`self.AllPlates`) (+ _returnvalue 1))))))

(fn `SetPuzzlePlates`
  (bind _puzzlearea (`self.PuzzleArea`))
  (if (`self.bOrderChangeable`)
    (`KismetArrayLibrary.Array_Clear` (`self.AllPlates`))
    (bind _outactors (`KismetSystemLibrary.ComponentOverlapActors` _puzzlearea (`SceneComponent.K2_GetComponentToWorld` _puzzlearea) (`|MakeArray` "ObjectTypeQuery1" "ObjectTypeQuery2" "ObjectTypeQuery3" "ObjectTypeQuery4" :!type "EObjectTypeQuery Enum") "/Game/Blueprints/Plates/OlderLogics/BP_Plate_AreaMethod.BP_Plate_AreaMethod_C"))
    (for _array_element _outactors
      (bind _asbp_plate_area_method (cast `/Game/Blueprints/Plates/OlderLogics/BP_Plate_AreaMethod` _array_element))
      (`self.AddPlate` _asbp_plate_area_method))
    (`self.Set Plate Numbers`)))

(fn `UserConstructionScript`
  (bind _activable (`self.Activable`))
  (bind _returnvalue (`KismetSystemLibrary.GetDisplayName` _activable))
  (`self.Set Plate Numbers`)
  (`/Engine/EditorBlueprintResources/StandardMacros.IsValid` _activable
    (:`Is Valid`
      (cast `/Game/Blueprints/Interfaces/BPI_Activable` _activable
        (:`then`
          (`/Engine/EditorBlueprintResources/StandardMacros.DoOnce` false
            (:`Completed`
              (`KismetSystemLibrary.PrintString` (`KismetStringLibrary.Concat_StrStr` _returnvalue ":: Inherits Activable Interface") true true (struct :`G` 0.66 :`B` 1.0 :`A` 1.0) 20.0))))
        (:`CastFailed`
          (`KismetSystemLibrary.PrintString` (`KismetStringLibrary.Concat_StrStr` _returnvalue ":: Does not Inherit from Activable Interface") true true (struct :`R` 1.0 :`A` 1.0) 20.0)
          (set `self.Activable` null))))))