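; Basic manager for a pressure or puzzle plate group that resets its plates and triggers a target object when the puzzle completes.
; The Construction Script registers the manager on every plate in AllPlates.
; ResetPlates deactivates all plates, and CompletePuzzle sends ActivateMessage to Activable; neither decides when the puzzle is solved.
; A check that Activable implements BPI_Activable exists but is disconnected.
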(fn `CompletePuzzle`
  (message `/Game/Blueprints/Interfaces/BPI_Activable.Activate` (`self.Activable`)))

(fn `ResetPlates`
  (for _array_element (`self.AllPlates`)
    (`/Game/Blueprints/Plates/OlderLogics/BP_Plate_Basic.Deactivate` _array_element)))

(fn `UserConstructionScript`
  (for _array_element (`self.AllPlates`)
    (`/Game/Blueprints/Plates/OlderLogics/BP_Plate_Basic.SetPlatesManager` _array_element self)))