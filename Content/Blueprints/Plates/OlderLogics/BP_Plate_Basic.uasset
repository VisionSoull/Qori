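; Pressure plate for an ordered step-on puzzle, numbered by a text render and coordinated by BP_PlatesManager_Basic.
; Player overlap on an active plate activates NextPlate, or completes the puzzle through the manager if final.
; Stepping on an inactive plate, or activating an already active one, makes the manager reset all plates.
; The construction script activates only the first plate, which ignores Deactivate; active state swaps the cube material.
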(event `self.ReceiveBeginPlay`
  (cast `/Game/Blueprints/Plates/OlderLogics/BP_PlatesManager_Basic` (`self.PlatesManager`))
  (`KismetSystemLibrary.PrintString` (`KismetStringLibrary.Concat_StrStr` (`KismetStringLibrary.Concat_StrStr` (`KismetSystemLibrary.GetDisplayName` self) ":: Succefully connected to ") (`KismetSystemLibrary.GetDisplayName` (`self.PlatesManager`))) true true (struct :`G` 1.0 :`B` 0.1519 :`A` 1.0) 20.0))

(event `self.Collider.OnComponentBeginOverlap`
  (params (OverlappedComponent :type "PrimitiveComponent Object Reference") (OtherActor :type "Actor Object Reference") (OtherComp :type "PrimitiveComponent Object Reference") (OtherBodyIndex :type Integer) (bFromSweep :type Boolean) (SweepResult :type "HitResult Structure (by ref)"))
  (if (== OtherActor (`GameplayStatics.GetPlayerPawn` 0))
    (if (`self.bInteractable`)
      (`KismetSystemLibrary.PrintString` "Detected Player")
      (if (`self.bIsActive`)
        (if (`self.bIsFinal`)
          (`/Game/Blueprints/Plates/OlderLogics/BP_PlatesManager_Basic.CompletePuzzle` (`self.PlatesManager`))
          (`KismetSystemLibrary.PrintString` "Completed Puzzle!")
          (else
            (`self.SetActive` (`self.NextPlate`))))
        (else
          (`/Game/Blueprints/Plates/OlderLogics/BP_PlatesManager_Basic.ResetPlates` (`self.PlatesManager`)))))))

(fn `Deactivate`
  (if (not (`self.bIsFirstPlate`))
    (set `self.bIsActive` false)
    (`self.SetActiveMaterial` (`self.bIsActive`))))

(fn `SetActive`
  (if (not (`self.bIsActive`))
    (set `self.bIsActive` true)
    (`self.SetActiveMaterial` (`self.bIsActive`))
    (else
      (`/Game/Blueprints/Plates/OlderLogics/BP_PlatesManager_Basic.ResetPlates` (`self.PlatesManager`)))))

(fn `SetActiveMaterial`
  (params (bActive :type Boolean))
  (if bActive
    (`PrimitiveComponent.SetMaterial` (`self.Cube`) 0 (`self.MaterialActive`))
    (else
      (`PrimitiveComponent.SetMaterial` (`self.Cube`) 0 (`self.MaterialNormal`)))))

(fn `SetNotInteractable`
  (set `self.bInteractable` false))

(fn `SetPlatesManager`
  (params (PlatesManager :type "/Game/Blueprints/Plates/OlderLogics/BP_PlatesManager_Basic Object Reference"))
  (set `self.PlatesManager` PlatesManager))

(fn `UserConstructionScript`
  (`TextRenderComponent.K2_SetText` (`self.TextRender`) (`KismetTextLibrary.Conv_IntToText` (`self.PlateNumber`)))
  (if (`self.bIsFirstPlate`)
    (set `self.bIsActive` true)
    (else
      (set `self.bIsActive` false)))
  (`self.SetActiveMaterial` (`self.bIsActive`))
  (`KismetSystemLibrary.PrintString` "Hello"))