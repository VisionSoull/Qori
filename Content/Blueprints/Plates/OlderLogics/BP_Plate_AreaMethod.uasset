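; A numbered floor plate for a sequence puzzle run by BP_PlatesManager_AreaMethod.
; Its construction script registers it with managers overlapping its cube, or unregisters it and zeroes its number when none overlap.
; A player overlap on an interactable plate asks the manager to activate the next plate if this one is active, otherwise to reset.
; Number and active state drive the text and material, with plate one starting active.
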(event `self.ReceiveBeginPlay`
  (cast `/Game/Blueprints/Plates/OlderLogics/BP_PlatesManager_AreaMethod` (`self.PlatesManager`)
    (:`then`
      (`KismetSystemLibrary.PrintString` (`KismetStringLibrary.Concat_StrStr` (`KismetStringLibrary.Concat_StrStr` (`KismetSystemLibrary.GetDisplayName` self) ":: Succefully connected to ") (`KismetSystemLibrary.GetDisplayName` (`self.PlatesManager`))) true true (struct :`G` 1.0 :`B` 0.1519 :`A` 1.0) 20.0))
    (:`CastFailed`
      (`KismetSystemLibrary.PrintString` (`KismetStringLibrary.Concat_StrStr` (`KismetSystemLibrary.GetDisplayName` self) ":: Not Connected to Plates Manager") true true (struct :`R` 1.0 :`G` 0.04617 :`A` 1.0) 20.0))))

(event `self.Collider.OnComponentBeginOverlap`
  (params (OverlappedComponent :type "PrimitiveComponent Object Reference") (OtherActor :type "Actor Object Reference") (OtherComp :type "PrimitiveComponent Object Reference") (OtherBodyIndex :type Integer) (bFromSweep :type Boolean) (SweepResult :type "HitResult Structure (by ref)"))
  (if (== OtherActor (`GameplayStatics.GetPlayerPawn` 0))
    (if (`self.bInteractable`)
      (if (`self.bIsActive`)
        (`/Game/Blueprints/Plates/OlderLogics/BP_PlatesManager_AreaMethod.SetNextPlateActive` (`self.PlatesManager`) null)
        (else
          (`/Game/Blueprints/Plates/OlderLogics/BP_PlatesManager_AreaMethod.ResetPlates` (`self.PlatesManager`)))))))

(fn `Deactivate`
  (if (not false)
    (set `self.bIsActive` false)
    (`self.SetActiveMaterial` (`self.bIsActive`))))

(fn `SetActive`
  (if (not (`self.bIsActive`))
    (set `self.bIsActive` true)
    (`self.SetActiveMaterial` (`self.bIsActive`))
    (else
      (`/Game/Blueprints/Plates/OlderLogics/BP_PlatesManager_AreaMethod.ResetPlates` (`self.PlatesManager`)))))

(fn `SetActiveMaterial`
  (params (bActive :type Boolean))
  ;[1 1 1] Sets the material corresponding to the plate's active state.
  (if bActive
    (`PrimitiveComponent.SetMaterial` (`self.Cube`) 0 (`self.MaterialActive`))
    (else
      (`PrimitiveComponent.SetMaterial` (`self.Cube`) 0 (`self.MaterialNormal`)))))

(fn `SetNotInteractable`
  (set `self.bInteractable` false))

(fn `SetNumber`
  (params (Number :type Integer))
  (bind _output_get (set `self.PlateNumber` Number))
  (`TextRenderComponent.K2_SetText` (`self.TextRender`) (`KismetTextLibrary.Conv_IntToText` _output_get))
  ;[1 1 1] If the plate number is one, it means that it is the first one in the puzzle and Is Active.
  (if (== (`self.PlateNumber`) 1)
    (set `self.bIsActive` true)
    (else
      (set `self.bIsActive` false)))
  (`self.SetActiveMaterial` (`self.bIsActive`)))

(fn `SetPlatesManager`
  (params (PlatesManager :type "/Game/Blueprints/Plates/OlderLogics/BP_PlatesManager_AreaMethod Object Reference"))
  (set `self.PlatesManager` PlatesManager))

(fn `UserConstructionScript`
  (bind _cube (`self.Cube`))
  (bind (_outactors _returnvalue) (`KismetSystemLibrary.ComponentOverlapActors` _cube (`SceneComponent.K2_GetComponentToWorld` _cube) (`|MakeArray` "ObjectTypeQuery1" "ObjectTypeQuery2" "ObjectTypeQuery3" "ObjectTypeQuery4" :!type "EObjectTypeQuery Enum") "/Game/Blueprints/Plates/OlderLogics/BP_PlatesManager_AreaMethod.BP_PlatesManager_AreaMethod_C"))
  (if _returnvalue
    (bind _output_get (set `self.Overlappingmanagers` _outactors))
    (for _array_element _output_get
      (bind _asbp_plates_manager_area_method (cast `/Game/Blueprints/Plates/OlderLogics/BP_PlatesManager_AreaMethod` _array_element))
      (`/Game/Blueprints/Plates/OlderLogics/BP_PlatesManager_AreaMethod.AddPlate` _asbp_plates_manager_area_method self))
    (else
      (for _array_element_2 (`self.Overlappingmanagers`)
        (bind _asbp_plates_manager_area_method_2 (cast `/Game/Blueprints/Plates/OlderLogics/BP_PlatesManager_AreaMethod` _array_element_2))
        (`/Game/Blueprints/Plates/OlderLogics/BP_PlatesManager_AreaMethod.RemovePlate` _asbp_plates_manager_area_method_2 self))
      (`KismetArrayLibrary.Array_Clear` (`self.Overlappingmanagers`))
      (`self.SetNumber` 0))))