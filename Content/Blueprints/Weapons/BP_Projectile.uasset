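; Weapon actor, despite the Projectile name, that damages BPI_Damageable actors on capsule hits when exactly one of wielder and target is an enemy.
; SetupWeapon supplies wielder and damage; IsAttacking toggles capsule overlap events and a socket-attached Niagara trail, clearing the once-per-target hit list when off.
; DetachWeapon drops the mesh into physics simulation.
; WeaponDecay fades its dynamic material by timeline, then destroys it.
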(event `self.ReceiveBeginPlay`
  ;[1 1 1] Attack Weapon Trail Niagara Particle System to the weapon socket that starts with "Trail"
  (for _array_element (`SceneComponent.GetAllSocketNames` (`self.StaticMesh`))
    (if (`KismetStringLibrary.StartsWith` (`KismetStringLibrary.Conv_NameToString` _array_element) "Trail")
      (`|ExecutionSequence`
        (:`then_0`
          (break))
        (:`then_1`
          (bind _returnvalue (`NiagaraFunctionLibrary.SpawnSystemAttached` (`self.TrailParticleEffect`) (`self.StaticMesh`) _array_element (0.0 0.0 0.0) (struct) "SnapToTarget"))
          (set `self.TrailParticle` _returnvalue)
          (`FXSystemComponent.SetFloatParameter` (`self.TrailParticle`) "TrailWidth" (`self.WeaponTrailWidth`))
          (`self.IsAttacking` false))))))

(event `self.Capsule.OnComponentHit`
  (params (HitComponent :type "PrimitiveComponent Object Reference") (OtherActor :type "Actor Object Reference") (OtherComp :type "PrimitiveComponent Object Reference") (NormalImpulse :type "Vector Structure") (Hit :type "HitResult Structure (by ref)"))
  (bind (_asbpi_damageable _bsuccess) (cast `/Game/Blueprints/DamageSystem/BPI_Damageable` OtherActor :!pure true))
  (bind _wielder (`self.Wielder`))
  ;[0.5052 0.2532 0.3738] Verify overlaps against actors that are not enemies and give damage to them. The Weapon Blueprints are only used by enemies.
  (if (and (and _bsuccess (!= OtherActor _wielder)) (!= (`KismetMathLibrary.ClassIsChildOf` (`GameplayStatics.GetObjectClass` _wielder) "/Game/Blueprints/Enemy/BP_Enemy_Base.BP_Enemy_Base_C") (`KismetMathLibrary.ClassIsChildOf` (`GameplayStatics.GetObjectClass` OtherActor) "/Game/Blueprints/Enemy/BP_Enemy_Base.BP_Enemy_Base_C")))
    (if (not (`KismetArrayLibrary.Array_Contains` (`self.HitTargets`) _asbpi_damageable))
      (`KismetArrayLibrary.Array_AddUnique` (`self.HitTargets`) _asbpi_damageable)
      (`/Game/Blueprints/DamageSystem/BPI_Damageable.TakeDamage` _asbpi_damageable (`self.AttackDamage`) (`self.Wielder`) (`.Location` (`GameplayStatics.BreakHitResult` Hit))))))

(event `WeaponDecay`
  (params (AfterDeathStartDecay :type "Float (single-precision)") (DecayTim :type "Float (double-precision)"))
  ;[0.1875 0.1875 0.1875] Decay over time
  (`KismetSystemLibrary.Delay` AfterDeathStartDecay)
  (`TimelineComponent.SetPlayRate` (`self.WeaponFade`) (/ 1.0 DecayTim))
  (bind (_direction _fade) (`Timeline|WeaponFade` :!via `PlayFromStart`)
    (:`Update`
      (`MaterialInstanceDynamic.SetScalarParameterValue` (`self.MeshMaterial`) "Fade" _fade))
    (:`Finished`
      (`KismetSystemLibrary.Delay` 0.2)
      (`self.K2_DestroyActor`))))

(fn `DetachWeapon`
  (bind _staticmesh (`self.StaticMesh`))
  (`self.IsAttacking` false)
  (`self.K2_DetachFromActor` "KeepWorld" "KeepWorld" "KeepWorld")
  (`PrimitiveComponent.SetSimulatePhysics` _staticmesh true)
  (`PrimitiveComponent.SetCollisionEnabled` _staticmesh "PhysicsOnly"))

(fn `IsAttacking`
  (params (bAttacking :type Boolean))
  (if bAttacking
    (`self.OverlapEvent` true)
    (`self.SetTrailActive` true)
    (else
      (`self.OverlapEvent` false)
      (`self.SetTrailActive` false)
      (`KismetArrayLibrary.Array_Clear` (`self.HitTargets`)))))

(fn `SetTrailActive`
  (params (bActive :type Boolean))
  (`ActorComponent.SetActive` (`self.TrailParticle`) bActive false))

(fn `SetupWeapon`
  (params (Wielder :type "Actor Object Reference") (AttackDamage :type Integer))
  (set `self.Wielder` Wielder)
  (set `self.AttackDamage` AttackDamage))

(fn `SetVisibility`
  (params (bNewVisibility :type Boolean))
  (`SceneComponent.SetVisibility` (`self.StaticMesh`) bNewVisibility false))

(fn `UserConstructionScript`
  (bind _staticmesh (`self.StaticMesh`))
  (bind _returnvalue (`PrimitiveComponent.CreateDynamicMaterialInstance` _staticmesh 0 (`PrimitiveComponent.GetMaterial` _staticmesh 0) "None"))
  (set `self.MeshMaterial` _returnvalue))