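; Game mode for Qori that owns the player's UI: HUD, death, pause and end-of-game menus.
; On BeginPlay it creates all four widgets, binding the HUD to the player pawn as its damageable actor and hiding the menus.
; Events show or hide each widget, with PauseMenu also toggling game pause, swapping out the HUD and setting Game-and-UI input.
; SetInfoText forwards messages to the HUD; DeadMenuHandler is an empty stub.
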(event `self.ReceiveBeginPlay`
  (`|ExecutionSequence`
    (:`then_0`
      (bind _asbp_player (cast `/Game/Blueprints/Player/BP_Player` (`GameplayStatics.GetPlayerPawn` 0)))
      (bind _returnvalue (`|CreateWidget` "/Game/UI/WBP_HUD.WBP_HUD_C" (`GameplayStatics.GetPlayerController` 0) _asbp_player))
      (bind _output_get (set `self.HUDWidget` _returnvalue))
      (`UserWidget.AddToViewport` _output_get 0))
    (:`then_1`
      (bind _returnvalue_2 (`|CreateWidget` "/Game/UI/WBP_DeadMenu.WBP_DeadMenu_C" (`GameplayStatics.GetPlayerController` 0)))
      (bind _output_get_2 (set `self.DeadMenuWidget` _returnvalue_2))
      (`UserWidget.AddToViewport` _output_get_2 0)
      (`Widget.SetVisibility` _output_get_2 "Hidden"))
    (:`then_2`
      (bind _returnvalue_3 (`|CreateWidget` "/Game/UI/WBP_PauseMenu.WBP_PauseMenu_C" (`GameplayStatics.GetPlayerController` 0)))
      (bind _output_get_3 (set `self.PauseMenuWidget` _returnvalue_3))
      (`UserWidget.AddToViewport` _output_get_3 0)
      (`Widget.SetVisibility` _output_get_3 "Hidden"))
    (:`then_3`
      (bind _returnvalue_4 (`|CreateWidget` "/Game/UI/WBP_EndMenu.WBP_EndMenu_C" (`GameplayStatics.GetPlayerController` 0)))
      (bind _output_get_4 (set `self.EndMenuWidget` _returnvalue_4))
      (`UserWidget.AddToViewport` _output_get_4 0)
      (`Widget.SetVisibility` _output_get_4 "Hidden"))))

(event `/Game/Blueprints/Interfaces/BPI_MenuHandler.PauseMenu`
  (bind _pausemenuwidget (`self.PauseMenuWidget`))
  (if (`Widget.IsVisible` (`self.PauseMenuWidget`))
    (`GameplayStatics.SetGamePaused` false)
    (`Widget.SetVisibility` _pausemenuwidget "Hidden")
    (`Widget.SetVisibility` (`self.HUDWidget`) "Visible")
    (else
      (`GameplayStatics.SetGamePaused` true)
      (`Widget.SetVisibility` _pausemenuwidget "Visible")
      (`Widget.SetVisibility` (`self.HUDWidget`) "Hidden")
      ;[1 1 1] Questions here
      (`WidgetBlueprintLibrary.SetInputMode_GameAndUIEx` (`GameplayStatics.GetPlayerController` 0) (`self.PauseMenuWidget`) "DoNotLock" false))))

(event `/Game/Blueprints/Interfaces/BPI_MenuHandler.DeadMenu`
  (params (bOpen :type Boolean))
  (bind _deadmenuwidget (`self.DeadMenuWidget`))
  (if bOpen
    (`Widget.SetVisibility` _deadmenuwidget "Visible")
    (else
      (`Widget.SetVisibility` _deadmenuwidget "Hidden"))))

(event `/Game/Blueprints/Interfaces/BPI_MenuHandler.EndMenu`
  (params (bOpen :type Boolean))
  (bind _endmenuwidget (`self.EndMenuWidget`))
  (if bOpen
    (`Widget.SetVisibility` _endmenuwidget "Visible")
    (else
      (`Widget.SetVisibility` _endmenuwidget "Hidden"))))

(event `/Game/Blueprints/Interfaces/BPI_MenuHandler.HUD`
  (params (bOpen :type Boolean))
  (bind _hudwidget (`self.HUDWidget`))
  (if bOpen
    (`Widget.SetVisibility` _hudwidget "Visible")
    (else
      (`Widget.SetVisibility` _hudwidget "Hidden"))))

(fn `DeadMenuHandler`
  (params (bOpen :type Boolean)))

(fn `SetInfoText`
  (params (InfoText :type Text))
  (`/Game/UI/WBP_HUD.SetInfoText` (`self.HUDWidget`) InfoText))

(fn `UserConstructionScript`)